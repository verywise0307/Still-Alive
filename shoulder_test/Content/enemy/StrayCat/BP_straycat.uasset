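; BP_straycat is an enemy stray cat that patrols between two named waypoints until it spots the player.
; Each tick it moves to the game instance's catnip ball if Toy is set, else to its patrol point while Straying, else to the player.
; Overlapping waypoints switches the destination.
; PawnSensing clears Straying, never restored here, only when a looping line trace to the player's head socket is unblocked.
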(event OnSeePawn(PawnSensing)
  (params (Pawn :type Pawn%20Object%20Reference))
  (Utilities|Casting|CastToBP_SuperSideScroller_MainCharacter Pawn)
  (if (Variables|Default|Getisseeingplayer)
    (Variables|Default|Setstraying false)))

(event OnPerceptionUpdated(AIPerception)
  (params (UpdatedActors :type Array%20of%20Actor%20Object%20References)))

(event Custom|Follow%20player
  (AI|AIMoveTo self "0, 0, 0" (Game|Player|GetPlayerPawn 0) 5.0 false))

(event EventBeginPlay
  (bind _point1 (Variables|Default|Getpoint1))
  (Utilities|Time|SetTimerbyFunctionName 0 "CheckVisibility" 0.1 true)
  (bind _outactors (Actor|GetAllActorsOfClass "/Game/enemy/StrayCat/BP_straycatpoint.BP_straycatpoint_C"))
  (for _array_element _outactors
    (if (Utilities|Enum|Equal(Enum) (Variables|/Game/enemy/StrayCat/BP_straycatpoint.BP_straycatpoint_C|Getpointname _array_element) _point1)
      (Variables|Default|SetBP_point1 _array_element)
      (Variables|Default|Setdestination _point1)
      (elif (Utilities|Enum|Equal(Enum) (Variables|/Game/enemy/StrayCat/BP_straycatpoint.BP_straycatpoint_C|Getpointname _array_element) (Variables|Default|Getpoint2))
        (Variables|Default|SetBP_point2 _array_element)))))

(event Collision|EventActorBeginOverlap
  (params (OtherActor :type Actor%20Object%20Reference))
  (bind _asbp_straycatpoint (Utilities|Casting|CastToBP_straycatpoint OtherActor))
  (if (Utilities|Enum|Equal(Enum) (Variables|/Game/enemy/StrayCat/BP_straycatpoint.BP_straycatpoint_C|Getpointname _asbp_straycatpoint) (Variables|Default|Getpoint1))
    (Variables|Default|Setdestination (Variables|Default|Getpoint2))
    (else
      (Variables|Default|Setdestination (Variables|Default|Getpoint1)))))

(event EventTick
  (params (DeltaSeconds :type Float%20%28single-precision%29))
  (bind _asgi_stage (Utilities|Casting|CastToGI_stage (Game|GetGameInstance)))
  (if (Variables|/Game/MainCharacter/Blueprints/GI_stage.GI_stage_C|Gettoy _asgi_stage)
    (AI|AIMoveTo self "0, 0, 0" (Variables|/Game/MainCharacter/Blueprints/GI_stage.GI_stage_C|Getcatnipball _asgi_stage) 5.0 false)
    (elif (Variables|Default|Getstraying)
      (if (Utilities|Enum|Equal(Enum) (Variables|Default|Getdestination) (Variables|Default|Getpoint1))
        (AI|AIMoveTo self "0, 0, 0" (Variables|Default|GetBP_point1) 5.0 false)
        (else
          (AI|AIMoveTo self "0, 0, 0" (Variables|Default|GetBP_point2) 5.0 false)))
      (else
        (AI|AIMoveTo self "0, 0, 0" (Game|Player|GetPlayerPawn 0) 5.0 false)))))

(fn ConstructionScript)

(fn CheckVisibility
  (bind _asbp_super_side_scroller_main_character (Utilities|Casting|CastToBP_SuperSideScroller_MainCharacter (Game|GetPlayerCharacter 0)))
  (bind _returnvalue (Collision|LineTraceByChannel (Transformation|GetActorLocation) (Transformation|GetSocketLocation (Variables|/Script/Engine.Character|GetMesh _asbp_super_side_scroller_main_character) "HeadTop_End소켓") "TraceTypeQuery1" false 0 "None"))
  (if _returnvalue
    (Variables|Default|Setisseeingplayer false)
    (else
      (Variables|Default|Setisseeingplayer true))))