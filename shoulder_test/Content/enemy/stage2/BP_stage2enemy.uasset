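; Stage 2 enemy that alternates between a yarn-throwing phase and a non-throwing phase on a looping timer.
; While alive and throwing, Tick spawns BP_throwingyarn with randomized position, yaw and speed, using a Doing flag and Delay to space out shots.
; The toyhit event briefly raises a Damage flag; HP is only read here, never reduced.
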(event Custom|toyhit
  (Variables|Default|Setdamage true)
  (Utilities|FlowControl|Delay 0.5)
  (Variables|Default|Setdamage false))

(event EventBeginPlay
  (Utilities|Time|SetTimerbyFunctionName 0 "switch state" 1e+01 true))

(event Collision|EventActorBeginOverlap
  (params (OtherActor :type Actor%20Object%20Reference)))

(event EventTick
  (params (DeltaSeconds :type Float%20%28single-precision%29))
  (bind _returnvalue (Transformation|GetActorTransform))
  (if (> (Variables|Default|GetHP) 0)
    (if (Variables|Default|Getthrow)
      (if (not (Variables|Default|Getdoing))
        (Variables|Default|Setdoing true)
        (bind _returnvalue_2 (Game|SpawnActorfromClass "/Game/enemy/stage2/BP_throwingyarn.BP_throwingyarn_C" (Math|Transform|MakeTransform (Math|Vector|MakeVector (+ (.x (.location _returnvalue)) (Variables|Default|Gety)) (+ (Math|Random|RandomFloatinRange -5e+02 5e+02) (.y (.location _returnvalue))) (+ (.z (.location _returnvalue)) (Variables|Default|Getheight) (Math|Random|RandomFloatinRange 0.0 2e+02))) (Math|Rotator|MakeRotator 0.0 0.0 (+ (.yaw (.rotation _returnvalue)) (Math|Random|RandomFloatinRange -2e+01 2e+01))) "2.500000,2.500000,2.500000") "Undefined" 0 0))
        (Variables|/Script/Engine.ProjectileMovementComponent|SetInitialSpeed (Variables|/Game/enemy/stage2/BP_throwingyarn.BP_throwingyarn_C|GetProjectileMovement _returnvalue_2) (Math|Random|RandomFloatinRange 2e+02 1e+03))
        (Utilities|FlowControl|Delay 1.0)
        (Variables|Default|Setdoing false)))))

(fn ConstructionScript)

(fn SwitchState
  (if (Variables|Default|Getthrow)
    (Variables|Default|Setthrow false)
    (Development|PrintString "비")
    (else
      (Variables|Default|Setthrow true)
      (Development|PrintString "던지기"))))