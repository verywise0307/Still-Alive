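; BP_stage2target is a stage 2 target that turns thrown toy hits into damage on the stage enemy.
; When a BP_throwingtoy overlaps its Sphere, it destroys the toy and increments the throwing hit count on GI_stage.
; It then finds every BP_stage2enemy in the level, lowers its HP, plays its hit audio if it survives, and calls its Toyhit.
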(event OnComponentBeginOverlap(Sphere)
  (params (OverlappedComponent :type Primitive%20Component%20Object%20Reference) (OtherActor :type Actor%20Object%20Reference) (OtherComp :type Primitive%20Component%20Object%20Reference) (OtherBodyIndex :type Integer) (bFromSweep :type Boolean) (SweepResult :type Hit%20Result%20Structure%20%28by%20ref%29))
  (bind _asbp_throwingtoy (Utilities|Casting|CastToBP_throwingtoy OtherActor))
  (Actor|DestroyActor _asbp_throwingtoy)
  (bind _asgi_stage (Utilities|Casting|CastToGI_stage (Game|GetGameInstance)))
  (Math|Integer|IncrementInt (Variables|/Game/MainCharacter/Blueprints/GI_stage.GI_stage_C|Getstage2throwingattackhitcount _asgi_stage)
    (:%20%20
      (bind _outactors (Actor|GetAllActorsOfClass "/Game/enemy/stage2/BP_stage2enemy.BP_stage2enemy_C"))
      (for _array_element _outactors
        (bind _output_get (Variables|/Game/enemy/stage2/BP_stage2enemy.BP_stage2enemy_C|SetHP _array_element (- (Variables|/Game/enemy/stage2/BP_stage2enemy.BP_stage2enemy_C|GetHP _array_element) 10)))
        (if (> _output_get 0)
          (Audio|Components|Audio|Play (Variables|/Game/enemy/stage2/BP_stage2enemy.BP_stage2enemy_C|GethitAudio _array_element) 0.0))
        (Default|Toyhit _array_element)))))

(event EventBeginPlay)

(event Collision|EventActorBeginOverlap
  (params (OtherActor :type Actor%20Object%20Reference)))

(event EventTick
  (params (DeltaSeconds :type Float%20%28single-precision%29)))

(fn ConstructionScript)