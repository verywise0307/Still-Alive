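; Stage 3 boss enemy: an invisible, periodically meowing stalker that chases the player outside side-scroll mode.
; The player's LightCone reveals it via SensorCapsule; 1.5 seconds of exposure costs it HP and relocates it randomly around its start.
; Touching the player deals damage and also relocates it.
; At zero HP it flags BP_bossbarrier as won, restores side view, records remaining lives in GI_stage and destroys itself.
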(event OnComponentBeginOverlap(Sphere)
  (params (OverlappedComponent :type Primitive%20Component%20Object%20Reference) (OtherActor :type Actor%20Object%20Reference) (OtherComp :type Primitive%20Component%20Object%20Reference) (OtherBodyIndex :type Integer) (bFromSweep :type Boolean) (SweepResult :type Hit%20Result%20Structure%20%28by%20ref%29))
  (bind _asbp_super_side_scroller_main_character (Utilities|Casting|CastToBP_SuperSideScroller_MainCharacter OtherActor))
  (if (== (Variables|/Game/MainCharacter/Blueprints/BP_SuperSideScroller_MainCharacter.BP_SuperSideScroller_MainCharacter_C|GetmainCapsule _asbp_super_side_scroller_main_character) OtherComp)
    (Variables|Default|Setcanattack true)
    (Variables|Default|Setattacking true)))

(event OnComponentEndOverlap(Sphere)
  (params (OverlappedComponent :type Primitive%20Component%20Object%20Reference) (OtherActor :type Actor%20Object%20Reference) (OtherComp :type Primitive%20Component%20Object%20Reference) (OtherBodyIndex :type Integer))
  (bind _asbp_super_side_scroller_main_character (Utilities|Casting|CastToBP_SuperSideScroller_MainCharacter OtherActor))
  (if (== (Variables|/Game/MainCharacter/Blueprints/BP_SuperSideScroller_MainCharacter.BP_SuperSideScroller_MainCharacter_C|GetmainCapsule _asbp_super_side_scroller_main_character) OtherComp)
    _))

(event OnComponentBeginOverlap(sensorCapsule)
  (params (OverlappedComponent :type Primitive%20Component%20Object%20Reference) (OtherActor :type Actor%20Object%20Reference) (OtherComp :type Primitive%20Component%20Object%20Reference) (OtherBodyIndex :type Integer) (bFromSweep :type Boolean) (SweepResult :type Hit%20Result%20Structure%20%28by%20ref%29))
  (bind _asbp_super_side_scroller_main_character (Utilities|Casting|CastToBP_SuperSideScroller_MainCharacter OtherActor))
  (if (== OtherComp (Variables|/Game/MainCharacter/Blueprints/BP_SuperSideScroller_MainCharacter.BP_SuperSideScroller_MainCharacter_C|GetlightCone _asbp_super_side_scroller_main_character))
    (Variables|Default|SetIsInLight true)
    (Rendering|SetVisibility (Variables|Character|GetMesh) true false)
    (Variables|Default|Setlightcountdown 0.0)
    (elif (and (== OtherComp (Variables|/Game/MainCharacter/Blueprints/BP_SuperSideScroller_MainCharacter.BP_SuperSideScroller_MainCharacter_C|GetmainCapsule _asbp_super_side_scroller_main_character)) (> (Variables|Default|GetHP) 0))
      (Variables|/Game/MainCharacter/Blueprints/BP_SuperSideScroller_MainCharacter.BP_SuperSideScroller_MainCharacter_C|SetHP _asbp_super_side_scroller_main_character (- (Variables|/Game/MainCharacter/Blueprints/BP_SuperSideScroller_MainCharacter.BP_SuperSideScroller_MainCharacter_C|GetHP _asbp_super_side_scroller_main_character) 10))
      (CallFunction|Newspawn2))))

(event OnComponentEndOverlap(sensorCapsule)
  (params (OverlappedComponent :type Primitive%20Component%20Object%20Reference) (OtherActor :type Actor%20Object%20Reference) (OtherComp :type Primitive%20Component%20Object%20Reference) (OtherBodyIndex :type Integer))
  (bind _asbp_super_side_scroller_main_character (Utilities|Casting|CastToBP_SuperSideScroller_MainCharacter OtherActor))
  (if (== OtherComp (Variables|/Game/MainCharacter/Blueprints/BP_SuperSideScroller_MainCharacter.BP_SuperSideScroller_MainCharacter_C|GetlightCone _asbp_super_side_scroller_main_character))
    (Variables|Default|SetIsInLight false)
    (Rendering|SetVisibility (Variables|Character|GetMesh) false false)
    (Variables|Default|Setlightcountdown 0.0)))

(event Custom|Newspawn2
  (bind _initlocation (Variables|Default|Getinitlocation))
  (bind _range (Variables|Default|Getrange))
  (bind _returnvalue (/ _range 2.0))
  (bind _returnvalue_2 (* -1.0 _returnvalue))
  (Variables|Default|Setattacking false)
  (Math|Random|SetRandomStreamSeed (Math|Random|MakeRandomStream (Math|Float|Truncate (Utilities|Time|GetGameTimeinSeconds))) 5)
  (Transformation|SetActorLocation (Math|Vector|MakeVector (+ (.x _initlocation) (Math|Random|RandomFloatinRange _returnvalue_2 _returnvalue)) (+ (.y _initlocation) (Math|Random|RandomFloatinRange _returnvalue_2 _returnvalue)) (.z _initlocation)) false false)
  (Utilities|FlowControl|Delay 1.5)
  (CallFunction|Playmeow)
  (Utilities|Time|SetTimerbyFunctionName 0 "playmeow" 5.0 true)
  (Variables|Default|SetIsInLight false)
  (Variables|Default|Setcanattack false)
  (Rendering|SetVisibility (Variables|Character|GetMesh) false false)
  (Variables|Default|SetHPsetting false))

(event EventBeginPlay
  (Variables|Default|Setinitlocation (Transformation|GetActorLocation))
  (Rendering|SetVisibility (Variables|Character|GetMesh) false false)
  (Utilities|Time|SetTimerbyFunctionName 0 "playmeow" 5.0 true))

(event Collision|EventActorBeginOverlap
  (params (OtherActor :type Actor%20Object%20Reference)))

(event EventTick
  (params (DeltaSeconds :type Float%20%28single-precision%29))
  (bind _returnvalue (Math|DateTime|Now))
  (bind _hp (Variables|Default|GetHP))
  (bind _returnvalue_2 (* (.hour _returnvalue) 3600))
  (bind _returnvalue_3 (* (.minute _returnvalue) 60))
  (bind _returnvalue_4 (+ _returnvalue_2 _returnvalue_3 (.second _returnvalue)))
  (bind _returnvalue_5 (Math|Conversions|ToFloat(Integer) _returnvalue_4))
  (bind _asbp_super_side_scroller_main_character (Utilities|Casting|CastToBP_SuperSideScroller_MainCharacter (Game|GetPlayerCharacter 0)))
  (if (not (Variables|/Script/shoulder_test.shoulder_testCharacter|Getsidescroll _asbp_super_side_scroller_main_character))
    (if (> (Variables|Default|GetHP) 0)
      (if (and (Variables|Default|Getcanattack) (not (Variables|Default|GetIsInLight)))
        _
        (else
          _))
      (Variables|Default|Setattacking false)
      (Variables|/Script/Engine.CharacterMovementComponent|SetMaxWalkSpeed (Variables|Character|GetCharacterMovement) 3e+02)
      (if (Variables|Default|GetIsInLight)
        (Variables|Default|Setlightcountdown (+ DeltaSeconds (Variables|Default|Getlightcountdown))))
      (AI|AIMoveTo self "0, 0, 0" (Game|Player|GetPlayerPawn 0) 5.0 false
        (:then
          (if (>= (Variables|Default|Getlightcountdown) 1.5)
            (Audio|Components|Audio|Play (Variables|Default|GetDamageAudio) 0.0)
            (if (not (Variables|Default|GetHPsetting))
              (Math|Integer|DecrementInt _hp
                (:%20%20
                  (bind _asgi_stage (Utilities|Casting|CastToGI_stage (Game|GetGameInstance)))
                  (if (== (Variables|/Game/MainCharacter/Blueprints/GI_stage.GI_stage_C|Getstage3firstattack _asgi_stage) 0.0)
                    (Variables|/Game/MainCharacter/Blueprints/GI_stage.GI_stage_C|Setstage3firstattack _asgi_stage _returnvalue_5)
                    (Variables|/Game/MainCharacter/Blueprints/GI_stage.GI_stage_C|Setstage3firstattacktime _asgi_stage (- _returnvalue_5 (Variables|/Game/MainCharacter/Blueprints/GI_stage.GI_stage_C|Getstage3bossstart _asgi_stage))))
                  (Variables|Default|SetHPsetting true)
                  (if (not (<= _hp 0))
                    (Utilities|FlowControl|Delay 1.0 :!label _label)
                    (CallFunction|NewSpawn))))
              (else
                (goto _label))))))
      (else
        (Components|Movement|StopMovementImmediately (Variables|Character|GetCharacterMovement))
        (Utilities|FlowControl|Delay 3.0)
        (bind _outactors (Actor|GetAllActorsOfClass "/Game/objects/bossstagebarrier/BP_bossbarrier.BP_bossbarrier_C"))
        (for _array_element _outactors
          (Variables|/Game/objects/bossstagebarrier/BP_bossbarrier.BP_bossbarrier_C|Setwin _array_element true)
          (bind _asbp_super_side_scroller_main_character_2 (Utilities|Casting|CastToBP_SuperSideScroller_MainCharacter (Game|GetPlayerCharacter 0)))
          (Variables|/Script/shoulder_test.shoulder_testCharacter|Setsidescroll _asbp_super_side_scroller_main_character_2 true)
          (Default|SwitchtoSideview _asbp_super_side_scroller_main_character_2)
          (bind _asgi_stage_2 (Utilities|Casting|CastToGI_stage (Game|GetGameInstance)))
          (Variables|/Game/MainCharacter/Blueprints/GI_stage.GI_stage_C|Setboss3remaininglives _asgi_stage_2 (/ (Variables|/Game/MainCharacter/Blueprints/BP_SuperSideScroller_MainCharacter.BP_SuperSideScroller_MainCharacter_C|GetHP _asbp_super_side_scroller_main_character_2) 10))
          (Actor|DestroyActor))))))

(fn ConstructionScript)

(fn Playmeow
  (Audio|Components|Audio|Play (Variables|Default|GetAudio) 0.0))

(fn NewSpawn
  (bind _initlocation (Variables|Default|Getinitlocation))
  (bind _range (Variables|Default|Getrange))
  (bind _returnvalue (/ _range 2.0))
  (bind _returnvalue_2 (* -1.0 _returnvalue))
  (Variables|Default|Setattacking false)
  (Math|Random|SetRandomStreamSeed (Math|Random|MakeRandomStream (Math|Float|Truncate (Utilities|Time|GetGameTimeinSeconds))) 5)
  (Transformation|SetActorLocation (Math|Vector|MakeVector (+ (.x _initlocation) (Math|Random|RandomFloatinRange _returnvalue_2 _returnvalue)) (+ (.y _initlocation) (Math|Random|RandomFloatinRange _returnvalue_2 _returnvalue)) (.z _initlocation)) false false)
  (Utilities|Time|SetTimerbyFunctionName 0 "playmeow" 1.0)
  (Variables|Default|SetIsInLight false)
  (Variables|Default|Setcanattack false)
  (Rendering|SetVisibility (Variables|Character|GetMesh) false false)
  (Variables|Default|SetHPsetting false))