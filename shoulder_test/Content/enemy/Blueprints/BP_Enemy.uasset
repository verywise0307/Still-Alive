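; BP_Enemy is a side-scroller enemy that picks a random attack when the main character is inside its Attackbox.
; Tick drives the timed cycle, gated by Attacking, and destroys the enemy after a delay once HP runs out.
; The fourth attack spawns a temporary Shockwave effect and directly subtracts player HP if Attack4 is set.
; Two ShockwaveBox overlaps toggle that flag, but only ShockwaveBox2 stores the Player reference.
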(event OnComponentBeginOverlap(ShockwaveBox2)
  (params (OverlappedComponent :type Primitive%20Component%20Object%20Reference) (OtherActor :type Actor%20Object%20Reference) (OtherComp :type Primitive%20Component%20Object%20Reference) (OtherBodyIndex :type Integer) (bFromSweep :type Boolean) (SweepResult :type Hit%20Result%20Structure%20%28by%20ref%29))
  (bind _asbp_super_side_scroller_main_character (Utilities|Casting|CastToBP_SuperSideScroller_MainCharacter OtherActor))
  (Variables|Default|SetAttack4 true)
  (Variables|Default|Setplayer _asbp_super_side_scroller_main_character))

(event OnComponentBeginOverlap(ShockwaveBox)
  (params (OverlappedComponent :type Primitive%20Component%20Object%20Reference) (OtherActor :type Actor%20Object%20Reference) (OtherComp :type Primitive%20Component%20Object%20Reference) (OtherBodyIndex :type Integer) (bFromSweep :type Boolean) (SweepResult :type Hit%20Result%20Structure%20%28by%20ref%29))
  (Utilities|Casting|CastToBP_SuperSideScroller_MainCharacter OtherActor)
  (Variables|Default|SetAttack4 true))

(event OnComponentEndOverlap(ShockwaveBox)
  (params (OverlappedComponent :type Primitive%20Component%20Object%20Reference) (OtherActor :type Actor%20Object%20Reference) (OtherComp :type Primitive%20Component%20Object%20Reference) (OtherBodyIndex :type Integer))
  (Utilities|Casting|CastToBP_SuperSideScroller_MainCharacter OtherActor)
  (Variables|Default|SetAttack4 false))

(event OnComponentEndOverlap(ShockwaveBox2)
  (params (OverlappedComponent :type Primitive%20Component%20Object%20Reference) (OtherActor :type Actor%20Object%20Reference) (OtherComp :type Primitive%20Component%20Object%20Reference) (OtherBodyIndex :type Integer))
  (Utilities|Casting|CastToBP_SuperSideScroller_MainCharacter OtherActor)
  (Variables|Default|SetAttack4 false))

(event EventBeginPlay)

(event Collision|EventActorBeginOverlap
  (params (OtherActor :type Actor%20Object%20Reference)))

(event EventTick
  (params (DeltaSeconds :type Float%20%28single-precision%29))
  (bind _player (Variables|Default|Getplayer))
  (if (Variables|Default|GetAttacking)
    (if (<= (Variables|Default|GetHP) 0)
      (Utilities|FlowControl|Delay 5.0)
      (Actor|DestroyActor))
    (else
      (for _array_element (Collision|GetOverlappingActors (Variables|Default|Getattackbox) 0 :!class /Script/Engine.PrimitiveComponent)
        (Utilities|Casting|CastToBP_SuperSideScroller_MainCharacter _array_element)
        (Variables|Default|SetAttack (Math|Random|RandomIntegerinRange 1 4))
        (Variables|Default|SetAttacking true)
        (if (== (Variables|Default|GetAttack) 4)
          (Utilities|FlowControl|Delay 1.5)
          (Variables|Default|SetAttack 5)
          (bind _returnvalue (Niagara|SpawnSystematLocation "/Game/enemy/Materials/shockwave.shockwave" (Transformation|GetWorldLocation (Variables|Default|GetShockwaveBox))))
          (if (Variables|Default|GetAttack4)
            (Variables|/Game/MainCharacter/Blueprints/BP_SuperSideScroller_MainCharacter.BP_SuperSideScroller_MainCharacter_C|SetHP _player (- (Variables|/Game/MainCharacter/Blueprints/BP_SuperSideScroller_MainCharacter.BP_SuperSideScroller_MainCharacter_C|GetHP _player) 30)))
          (Utilities|FlowControl|Delay 0.5)
          (Components|DestroyComponent _returnvalue)
          (Variables|Default|SetAttack 0)
          (Utilities|FlowControl|Delay 1.0)
          (Variables|Default|SetAttacking false)
          (if (<= (Variables|Default|GetHP) 0)
            (Utilities|FlowControl|Delay 5.0)
            (Actor|DestroyActor))
          (else
            (Utilities|FlowControl|Delay 2.5)
            (Variables|Default|SetAttack 0)
            (Utilities|FlowControl|Delay 0.5)
            (Variables|Default|SetAttacking false)
            (if (<= (Variables|Default|GetHP) 0)
              (Utilities|FlowControl|Delay 5.0)
              (Actor|DestroyActor))))))))

(fn ConstructionScript)