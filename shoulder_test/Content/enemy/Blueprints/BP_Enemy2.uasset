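; BP_Enemy2 is a boss enemy that chases and attacks the player, or diverts to the game instance's toy while active.
; Tick drives movement and, gated by Attacking and Select flags, picks one of four delayed attacks, one spawning a shockwave.
; AttackBox and Wavebox share one overlap flag that decides whether attacks damage the player.
; At zero HP it sets Win on boss barriers and destroys itself after a delay.
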(event OnComponentBeginOverlap(attackBox)
  (params (OverlappedComponent :type Primitive%20Component%20Object%20Reference) (OtherActor :type Actor%20Object%20Reference) (OtherComp :type Primitive%20Component%20Object%20Reference) (OtherBodyIndex :type Integer) (bFromSweep :type Boolean) (SweepResult :type Hit%20Result%20Structure%20%28by%20ref%29))
  (bind _asbp_super_side_scroller_main_character (Utilities|Casting|CastToBP_SuperSideScroller_MainCharacter OtherActor))
  (if (== (Variables|/Game/MainCharacter/Blueprints/BP_SuperSideScroller_MainCharacter.BP_SuperSideScroller_MainCharacter_C|GetmainCapsule _asbp_super_side_scroller_main_character) OtherComp)
    (Variables|Default|SetIsplayeroverlap true)))

(event OnComponentEndOverlap(attackBox)
  (params (OverlappedComponent :type Primitive%20Component%20Object%20Reference) (OtherActor :type Actor%20Object%20Reference) (OtherComp :type Primitive%20Component%20Object%20Reference) (OtherBodyIndex :type Integer))
  (bind _asbp_super_side_scroller_main_character (Utilities|Casting|CastToBP_SuperSideScroller_MainCharacter OtherActor))
  (if (== (Variables|/Game/MainCharacter/Blueprints/BP_SuperSideScroller_MainCharacter.BP_SuperSideScroller_MainCharacter_C|GetmainCapsule _asbp_super_side_scroller_main_character) OtherComp)
    (Variables|Default|SetIsplayeroverlap false)))

(event OnComponentBeginOverlap(wavebox)
  (params (OverlappedComponent :type Primitive%20Component%20Object%20Reference) (OtherActor :type Actor%20Object%20Reference) (OtherComp :type Primitive%20Component%20Object%20Reference) (OtherBodyIndex :type Integer) (bFromSweep :type Boolean) (SweepResult :type Hit%20Result%20Structure%20%28by%20ref%29))
  (bind _asbp_super_side_scroller_main_character (Utilities|Casting|CastToBP_SuperSideScroller_MainCharacter OtherActor))
  (if (== (Variables|/Game/MainCharacter/Blueprints/BP_SuperSideScroller_MainCharacter.BP_SuperSideScroller_MainCharacter_C|GetmainCapsule _asbp_super_side_scroller_main_character) OtherComp)
    (Variables|Default|SetIsplayeroverlap true)))

(event OnComponentEndOverlap(wavebox)
  (params (OverlappedComponent :type Primitive%20Component%20Object%20Reference) (OtherActor :type Actor%20Object%20Reference) (OtherComp :type Primitive%20Component%20Object%20Reference) (OtherBodyIndex :type Integer))
  (bind _asbp_super_side_scroller_main_character (Utilities|Casting|CastToBP_SuperSideScroller_MainCharacter OtherActor))
  (if (== (Variables|/Game/MainCharacter/Blueprints/BP_SuperSideScroller_MainCharacter.BP_SuperSideScroller_MainCharacter_C|GetmainCapsule _asbp_super_side_scroller_main_character) OtherComp)
    (Variables|Default|SetIsplayeroverlap false)))

(event EventBeginPlay)

(event Collision|EventActorBeginOverlap
  (params (OtherActor :type Actor%20Object%20Reference)))

(event EventTick
  (params (DeltaSeconds :type Float%20%28single-precision%29))
  (bind _returnvalue (Game|Player|GetPlayerPawn 0))
  (bind _returnvalue_2 (Transformation|GetActorLocation))
  (if (> (Variables|Default|GetHP) 0)
    (bind _asgi_stage (Utilities|Casting|CastToGI_stage (Game|GetGameInstance)))
    (if (and (Variables|/Game/MainCharacter/Blueprints/GI_stage.GI_stage_C|Gettoy _asgi_stage) (not (Variables|Default|Getattacking)))
      (AI|AIMoveTo self "0, 0, 0" (Variables|/Game/MainCharacter/Blueprints/GI_stage.GI_stage_C|GetBP_toy _asgi_stage) 5.0 false)
      (elif (and (> (Transformation|GetDistanceTo _returnvalue) 2e+02) (not (Variables|Default|Getattacking)))
        (AI|AIMoveTo self "0, 0, 0" _returnvalue 5.0 false)
        (else
          (Components|Movement|StopMovementImmediately (Variables|Character|GetCharacterMovement))
          (Variables|Default|Setattacking true)
          (if (not (Variables|Default|Getselect))
            (Variables|Default|Setselect true)
            (bind _output_get (Variables|Default|Setattack (Math|Random|RandomIntegerinRange 1 4)))
            (if (== _output_get 4)
              (Variables|Default|Setattack 4)
              (Utilities|FlowControl|Delay 2.0)
              (Variables|Default|Setattack 5)
              (bind _returnvalue_3 (Game|SpawnActorfromClass "/Game/enemy/Blueprints/BP_shockwave.BP_shockwave_C" (Math|Transform|MakeTransform (Math|Vector|MakeVector (.x _returnvalue_2) (.y _returnvalue_2) (- (.z _returnvalue_2) 1.5e+02)) "0, 0, 0" "1.000000,1.000000,1.000000") "Undefined" 0 0))
              (if (Variables|Default|GetIsplayeroverlap)
                (bind _asbp_super_side_scroller_main_character (Utilities|Casting|CastToBP_SuperSideScroller_MainCharacter (Game|GetPlayerCharacter 0)))
                (Variables|/Game/MainCharacter/Blueprints/BP_SuperSideScroller_MainCharacter.BP_SuperSideScroller_MainCharacter_C|SetHP _asbp_super_side_scroller_main_character (- (Variables|/Game/MainCharacter/Blueprints/BP_SuperSideScroller_MainCharacter.BP_SuperSideScroller_MainCharacter_C|GetHP _asbp_super_side_scroller_main_character) 10)))
              (Utilities|FlowControl|Delay 1.0)
              (Actor|DestroyActor _returnvalue_3)
              (Variables|Default|Setattacking false)
              (Variables|Default|Setattack 0)
              (Variables|Default|Setselect false)
              (else
                (bind _asbp_super_side_scroller_main_character_2 (Utilities|Casting|CastToBP_SuperSideScroller_MainCharacter (Game|GetPlayerCharacter 0)))
                (if (== _output_get 1)
                  (Utilities|FlowControl|Delay 1.0)
                  (if (Variables|Default|GetIsplayeroverlap) :!label _label
                    (Variables|/Game/MainCharacter/Blueprints/BP_SuperSideScroller_MainCharacter.BP_SuperSideScroller_MainCharacter_C|SetHP _asbp_super_side_scroller_main_character_2 (- (Variables|/Game/MainCharacter/Blueprints/BP_SuperSideScroller_MainCharacter.BP_SuperSideScroller_MainCharacter_C|GetHP _asbp_super_side_scroller_main_character_2) 10)))
                  (Utilities|FlowControl|Delay 1.0)
                  (Variables|Default|Setattacking false)
                  (Variables|Default|Setattack 0)
                  (Utilities|FlowControl|Delay 0.5)
                  (Variables|Default|Setselect false)
                  (elif (== _output_get 2)
                    (Utilities|FlowControl|Delay 1.0)
                    (goto _label)
                    (elif (== _output_get 3)
                      (Utilities|FlowControl|Delay 0.5)
                      (goto _label))))))))))
    (else
      (bind _outactors (Actor|GetAllActorsOfClass "/Game/objects/bossstagebarrier/BP_bossbarrier.BP_bossbarrier_C"))
      (for _array_element _outactors
        (Variables|/Game/objects/bossstagebarrier/BP_bossbarrier.BP_bossbarrier_C|Setwin _array_element true)
        (Utilities|FlowControl|Delay 5.0)
        (Actor|DestroyActor)))))

(fn ConstructionScript)