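; GI_stage is a Game Instance that holds playtest telemetry for three stages and their bosses: deaths, actions, timings, endings.
; Init enables logging and timestamps the session.
; Per-category functions append counters to one Fulllog string, clamping negative times and computing throw accuracy.
; The chain that deletes save slot "1", assembles and prints the log is disconnected; Shutdown is empty, Magiccirclelog is uncalled, and Bosstimelog never computes positive durations.
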(event EventShutdown)

(event EventInit
  (bind _returnvalue (Math|DateTime|Now))
  (bind (_year _month _day _hour _minute _second) (Math|DateTime|BreakDateTime _returnvalue))
  (Variables|Default|Setlog true)
  (Variables|Default|Setlogstart (Utilities|String|Append (Utilities|String|ToString(Integer) _year) "-" (Utilities|String|ToString(Integer) _month) "-" (Utilities|String|ToString(Integer) _day) " " (Utilities|String|ToString(Integer) _hour) ":" (Utilities|String|ToString(Integer) _minute) ":" (Utilities|String|ToString(Integer) _second))))

(fn Deathlog
  (Variables|Default|Setfulllog (Utilities|String|Append (Variables|Default|Getfulllog) " deathcount : " (Utilities|String|ToString(Integer) (Variables|Default|Getdeathcount))))
  (Variables|Default|Setfulllog (Utilities|String|Append (Variables|Default|Getfulllog) " stage1deathcount : " (Utilities|String|ToString(Integer) (Variables|Default|Getstage1deathcount))))
  (Variables|Default|Setfulllog (Utilities|String|Append (Variables|Default|Getfulllog) " stage2deathcount : " (Utilities|String|ToString(Integer) (Variables|Default|Getstage2deathcount))))
  (Variables|Default|Setfulllog (Utilities|String|Append (Variables|Default|Getfulllog) " stage3deathcount : " (Utilities|String|ToString(Integer) (Variables|Default|Getstage3deathcount))))
  (return))

(fn Playtimelog
  (bind _stage1endtime (Variables|Default|Getstage1endtime))
  (bind _stage1starttime (Variables|Default|Getstage1starttime))
  (bind _stage2starttime (Variables|Default|Getstage2starttime))
  (bind _stage2endtime (Variables|Default|Getstage2endtime))
  (bind _stage3endtime (Variables|Default|Getstage3endtime))
  (bind _stage3starttime (Variables|Default|Getstage3starttime))
  (bind _returnvalue (- _stage3endtime _stage3starttime))
  (bind _returnvalue_2 (- _stage1endtime _stage1starttime))
  (bind _returnvalue_3 (- _stage2endtime _stage2starttime))
  (if (< _returnvalue_2 0.0)
    (Variables|Default|Setstage1playtime 0.0)
    (else
      (Variables|Default|Setstage1playtime _returnvalue_2)))
  (if (< _returnvalue_3 0.0)
    (Variables|Default|Setstage2playtime 0.0)
    (else
      (Variables|Default|Setstage2playtime _returnvalue_3)))
  (if (< _returnvalue 0.0)
    (Variables|Default|Setstage3playtime 0.0)
    (else
      (Variables|Default|Setstage3playtime _returnvalue)))
  (Variables|Default|Setfulllog (Utilities|String|Append (Variables|Default|Getfulllog) " playtime : " (Utilities|String|ToString(Float) (+ (Variables|Default|Getstage1playtime) (Variables|Default|Getstage2playtime) (Variables|Default|Getstage3playtime)))))
  (Variables|Default|Setfulllog (Utilities|String|Append (Variables|Default|Getfulllog) " stage1playtime : " (Utilities|String|ToString(Float) (Variables|Default|Getstage1playtime))))
  (Variables|Default|Setfulllog (Utilities|String|Append (Variables|Default|Getfulllog) " stage2playtime : " (Utilities|String|ToString(Float) (Variables|Default|Getstage2playtime))))
  (Variables|Default|Setfulllog (Utilities|String|Append (Variables|Default|Getfulllog) " stage3playtime : " (Utilities|String|ToString(Float) (Variables|Default|Getstage3playtime))))
  (return))

(fn Jumplog
  (Variables|Default|Setfulllog (Utilities|String|Append (Variables|Default|Getfulllog) " jumpcount: " (Utilities|String|ToString(Integer) (Variables|Default|Getjumpcount))))
  (Variables|Default|Setfulllog (Utilities|String|Append (Variables|Default|Getfulllog) " stage1jumpcount :  " (Utilities|String|ToString(Integer) (Variables|Default|Getstage1jumpcount))))
  (Variables|Default|Setfulllog (Utilities|String|Append (Variables|Default|Getfulllog) " stage2jumpcount: " (Utilities|String|ToString(Integer) (Variables|Default|Getstage2jumpcount))))
  (Variables|Default|Setfulllog (Utilities|String|Append (Variables|Default|Getfulllog) " stage3jumpcount: " (Utilities|String|ToString(Integer) (Variables|Default|Getstage3jumpcount))))
  (return))

(fn Climbinglog
  (Variables|Default|Setfulllog (Utilities|String|Append (Variables|Default|Getfulllog) " climbingcount: " (Utilities|String|ToString(Integer) (Variables|Default|Gettotalclimbingcount))))
  (Variables|Default|Setfulllog (Utilities|String|Append (Variables|Default|Getfulllog) " stage1climbingcount :  " (Utilities|String|ToString(Integer) (Variables|Default|Getstage1climbingcount))))
  (Variables|Default|Setfulllog (Utilities|String|Append (Variables|Default|Getfulllog) " stage2climbingcount: " (Utilities|String|ToString(Integer) (Variables|Default|Getstage2climbingcount))))
  (Variables|Default|Setfulllog (Utilities|String|Append (Variables|Default|Getfulllog) " stage3climbingcount: " (Utilities|String|ToString(Integer) (Variables|Default|Getstage3climbingcount))))
  (return))

(fn Hanglog
  (Variables|Default|Setfulllog (Utilities|String|Append (Variables|Default|Getfulllog) " hangcount : " (Utilities|String|ToString(Integer) (Variables|Default|Gethangcount))))
  (Variables|Default|Setfulllog (Utilities|String|Append (Variables|Default|Getfulllog) " stage1hangcount :  " (Utilities|String|ToString(Integer) (Variables|Default|Getstage1hangcount))))
  (Variables|Default|Setfulllog (Utilities|String|Append (Variables|Default|Getfulllog) " stage2hangcount : " (Utilities|String|ToString(Integer) (Variables|Default|Getstage2hangcount))))
  (Variables|Default|Setfulllog (Utilities|String|Append (Variables|Default|Getfulllog) " stage3hangcount : " (Utilities|String|ToString(Integer) (Variables|Default|Getstage3hangcount))))
  (return))

(fn Attacklog
  (Variables|Default|Setfulllog (Utilities|String|Append (Variables|Default|Getfulllog) " attackcount : " (Utilities|String|ToString(Integer) (Variables|Default|Getattackcount))))
  (Variables|Default|Setfulllog (Utilities|String|Append (Variables|Default|Getfulllog) " stage1smashattackcount :  " (Utilities|String|ToString(Integer) (Variables|Default|Getstage1smashattackcount)) " stage1throwingattackcount : " (Utilities|String|ToString(Integer) (Variables|Default|Getstage1throwingattackcount)) " stage1throwingaccuracy : " (Utilities|String|ToString(Text) (Utilities|Text|ToText(Float) (/ (Math|Conversions|ToFloat(Integer) (Variables|Default|Getstage1throwingattackhitcount)) (Math|Conversions|ToFloat(Integer) (Variables|Default|Getstage1throwingattackcount))) "HalfToEven" false true 1 324 0 2))))
  (Variables|Default|Setfulllog (Utilities|String|Append (Variables|Default|Getfulllog) " stage2attackcount : " (Utilities|String|ToString(Integer) (Variables|Default|Getstage2attackcount)) " stage2throwingaccuracy : " (Utilities|String|ToString(Text) (Utilities|Text|ToText(Float) (/ (Math|Conversions|ToFloat(Integer) (Variables|Default|Getstage2throwingattackhitcount)) (Math|Conversions|ToFloat(Integer) (Variables|Default|Getstage2attackcount))) "HalfToEven" false true 1 324 0 2)) " bossyarnattackaccuracy : " (Utilities|String|ToString(Text) (Utilities|Text|ToText(Float) (/ (Math|Conversions|ToFloat(Integer) (Variables|Default|Getthrowingyarnhitcount)) (Math|Conversions|ToFloat(Integer) (Variables|Default|Getthrowingyarncount))) "HalfToEven" false true 1 324 0 2))))
  (return))

(fn Crouchlog
  (Variables|Default|Setfulllog (Utilities|String|Append (Variables|Default|Getfulllog) " crouchcount : " (Utilities|String|ToString(Integer) (Variables|Default|Getcrouchcount))))
  (Variables|Default|Setfulllog (Utilities|String|Append (Variables|Default|Getfulllog) " stage1crouchcount :  " (Utilities|String|ToString(Integer) (Variables|Default|Getstage1crouchcount))))
  (Variables|Default|Setfulllog (Utilities|String|Append (Variables|Default|Getfulllog) " stage2crouchcount : " (Utilities|String|ToString(Integer) (Variables|Default|Getstage2crouchcount))))
  (Variables|Default|Setfulllog (Utilities|String|Append (Variables|Default|Getfulllog) " stage3crouchcount : " (Utilities|String|ToString(Integer) (Variables|Default|Getstage3crouchcount))))
  (return))

(fn Pushlog
  (Variables|Default|Setfulllog (Utilities|String|Append (Variables|Default|Getfulllog) " pushcount : " (Utilities|String|ToString(Integer) (Variables|Default|Getpushcount))))
  (Variables|Default|Setfulllog (Utilities|String|Append (Variables|Default|Getfulllog) " stage1pushcount :  " (Utilities|String|ToString(Integer) (Variables|Default|Getstage1pushcount))))
  (Variables|Default|Setfulllog (Utilities|String|Append (Variables|Default|Getfulllog) " stage2pushcount : " (Utilities|String|ToString(Integer) (Variables|Default|Getstage2pushcount))))
  (Variables|Default|Setfulllog (Utilities|String|Append (Variables|Default|Getfulllog) " stage3pushcount : " (Utilities|String|ToString(Integer) (Variables|Default|Getstage3pushcount))))
  (return))

(fn Signlog
  (Variables|Default|Setfulllog (Utilities|String|Append (Variables|Default|Getfulllog) " signcount : " (Utilities|String|ToString(Integer) (Variables|Default|Getsignclickcount))))
  (Variables|Default|Setfulllog (Utilities|String|Append (Variables|Default|Getfulllog) " signclick1count :  " (Utilities|String|ToString(Integer) (Variables|Default|Getsignclick1count))))
  (Variables|Default|Setfulllog (Utilities|String|Append (Variables|Default|Getfulllog) " signclick2count : " (Utilities|String|ToString(Integer) (Variables|Default|Getsignclick2count))))
  (Variables|Default|Setfulllog (Utilities|String|Append (Variables|Default|Getfulllog) " signclick3count : " (Utilities|String|ToString(Integer) (Variables|Default|Getsignclick3count))))
  (return))

(fn Animlog
  (Variables|Default|Setfulllog (Utilities|String|Append (Variables|Default|Getfulllog) " animskipcount : " (Utilities|String|ToString(Integer) (Variables|Default|Getanimskipcount))))
  (Variables|Default|Setfulllog (Utilities|String|Append (Variables|Default|Getfulllog) " bossanim1skipcount :  " (Utilities|String|ToString(Integer) (Variables|Default|Getbossanim1count))))
  (Variables|Default|Setfulllog (Utilities|String|Append (Variables|Default|Getfulllog) " bossanim2skipcount : " (Utilities|String|ToString(Integer) (Variables|Default|Getbossanim2count))))
  (Variables|Default|Setfulllog (Utilities|String|Append (Variables|Default|Getfulllog) " bossanim3skipcount : " (Utilities|String|ToString(Integer) (Variables|Default|Getbossanim3count))))
  (return))

(fn Npcchatlog
  (Variables|Default|Setfulllog (Utilities|String|Append (Variables|Default|Getfulllog) " npcchat1 : " (Utilities|String|ToString(Integer) (Variables|Default|Getnpcchat1))))
  (Variables|Default|Setfulllog (Utilities|String|Append (Variables|Default|Getfulllog) " npcchat2 : " (Utilities|String|ToString(Integer) (Variables|Default|Getnpcchat2))))
  (Variables|Default|Setfulllog (Utilities|String|Append (Variables|Default|Getfulllog) " npcchat3 : " (Utilities|String|ToString(Integer) (Variables|Default|Getnpcchat3))))
  (return))

(fn Endinglog
  (Variables|Default|Setfulllog (Utilities|String|Append (Variables|Default|Getfulllog) " happyending : " (Utilities|String|ToString(Integer) (Variables|Default|Gethappyending))))
  (Variables|Default|Setfulllog (Utilities|String|Append (Variables|Default|Getfulllog) " sadending : " (Utilities|String|ToString(Integer) (Variables|Default|Getsadending))))
  (return))

(fn Bosstimelog
  (if (< (- (Variables|Default|Getstage1bossend) (Variables|Default|Getstage1bossstart)) 0.0)
    (Variables|Default|Setstage1bosstime 0.0))
  (if (< (- (Variables|Default|Getstage2bossend) (Variables|Default|Getstage2bossstart)) 0.0)
    (Variables|Default|Setstage2bosstime 0.0))
  (if (< (- (Variables|Default|Getstage3bossend) (Variables|Default|Getstage3bossstart)) 0.0)
    (Variables|Default|Setstage3bosstime 0.0))
  (Variables|Default|Setfulllog (Utilities|String|Append (Variables|Default|Getfulllog) " stage1bosstime : " (Utilities|String|ToString(Float) (Variables|Default|Getstage1bosstime))))
  (Variables|Default|Setfulllog (Utilities|String|Append (Variables|Default|Getfulllog) " stage2bosstime : " (Utilities|String|ToString(Float) (Variables|Default|Getstage2bosstime))))
  (Variables|Default|Setfulllog (Utilities|String|Append (Variables|Default|Getfulllog) " stage3bosstime : " (Utilities|String|ToString(Float) (Variables|Default|Getstage3bosstime))))
  (return))

(fn Bossfaillog
  (Variables|Default|Setfulllog (Utilities|String|Append (Variables|Default|Getfulllog) " bossfailcount : " (Utilities|String|ToString(Integer) (Variables|Default|Getbossstagefailcount))))
  (Variables|Default|Setfulllog (Utilities|String|Append (Variables|Default|Getfulllog) " boss1failcount : " (Utilities|String|ToString(Integer) (Variables|Default|Getbossstage1failcount))))
  (Variables|Default|Setfulllog (Utilities|String|Append (Variables|Default|Getfulllog) " boss2failcount : " (Utilities|String|ToString(Integer) (Variables|Default|Getbossstage2failcount))))
  (Variables|Default|Setfulllog (Utilities|String|Append (Variables|Default|Getfulllog) " boss3failcount : " (Utilities|String|ToString(Integer) (Variables|Default|Getbossstage3failcount))))
  (return))

(fn Pauselog
  (Variables|Default|Setfulllog (Utilities|String|Append (Variables|Default|Getfulllog) " pausecount : " (Utilities|String|ToString(Integer) (Variables|Default|Getpausecount))))
  (Variables|Default|Setfulllog (Utilities|String|Append (Variables|Default|Getfulllog) " pausecount1 : " (Utilities|String|ToString(Integer) (Variables|Default|Getpausecount1))))
  (Variables|Default|Setfulllog (Utilities|String|Append (Variables|Default|Getfulllog) " pausecount2 : " (Utilities|String|ToString(Integer) (Variables|Default|Getpausecount2))))
  (Variables|Default|Setfulllog (Utilities|String|Append (Variables|Default|Getfulllog) " pausecount3 : " (Utilities|String|ToString(Integer) (Variables|Default|Getpausecount3))))
  (return))

(fn Magiccirclelog
  (Variables|Default|Setfulllog (Utilities|String|Append (Variables|Default|Getfulllog) " magiccirclecount : " (Utilities|String|ToString(Integer) (Variables|Default|Getmagiccirclrcount))))
  (return))

(fn Bossfirstattacklog
  (if (< (Variables|Default|Getstage1firstattacktime) 0.0)
    (Variables|Default|Setstage1firstattacktime 0.0))
  (if (< (Variables|Default|Getstage2firstattacktime) 0.0)
    (Variables|Default|Setstage2firstattacktime 0.0))
  (if (< (Variables|Default|Getstage3firstattacktime) 0.0)
    (Variables|Default|Setstage3firstattacktime 0.0))
  (Variables|Default|Setfulllog (Utilities|String|Append (Variables|Default|Getfulllog) " stage1bossfirstattacktime : " (Utilities|String|ToString(Float) (Variables|Default|Getstage1firstattacktime))))
  (Variables|Default|Setfulllog (Utilities|String|Append (Variables|Default|Getfulllog) " stage2bossfirstattacktime : " (Utilities|String|ToString(Float) (Variables|Default|Getstage2firstattacktime))))
  (Variables|Default|Setfulllog (Utilities|String|Append (Variables|Default|Getfulllog) " stage3bossfirstattacktime : " (Utilities|String|ToString(Float) (Variables|Default|Getstage3firstattacktime))))
  (return))

(fn Itemlog
  (Variables|Default|Setfulllog (Utilities|String|Append (Variables|Default|Getfulllog) " itemcount: " (Utilities|String|ToString(Integer) (Variables|Default|Getitem))))
  (Variables|Default|Setfulllog (Utilities|String|Append (Variables|Default|Getfulllog) " item1 : " (Utilities|String|ToString(Integer) (Variables|Default|Getitem1))))
  (Variables|Default|Setfulllog (Utilities|String|Append (Variables|Default|Getfulllog) " item2 : " (Utilities|String|ToString(Integer) (Variables|Default|Getitem2))))
  (Variables|Default|Setfulllog (Utilities|String|Append (Variables|Default|Getfulllog) " item3 : " (Utilities|String|ToString(Integer) (Variables|Default|Getitem3))))
  (return))

(fn Bossliveslog
  (Variables|Default|Setfulllog (Utilities|String|Append (Variables|Default|Getfulllog) " boss1remaininglives : " (Utilities|String|ToString(Integer) (Variables|Default|Getboss1remaininglives))))
  (Variables|Default|Setfulllog (Utilities|String|Append (Variables|Default|Getfulllog) " boss2remaininglives : " (Utilities|String|ToString(Integer) (Variables|Default|Getboss2remaininglives))))
  (Variables|Default|Setfulllog (Utilities|String|Append (Variables|Default|Getfulllog) " boss3remaininglives : " (Utilities|String|ToString(Integer) (Variables|Default|Getboss3remaininglives))))
  (return))