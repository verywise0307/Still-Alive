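; Configurable leaf VFX actor that drives a Niagara component to show one of six leaf types as a burst or continuous spawn.
; The construction script pushes spawn, lifetime, scale, shape, wind, vortex and color settings into Niagara user parameters and creates a dynamic material for color intensity.
; Enum selections then swap leaf mesh and material, with Leaf 4–6 reusing the birch mesh, and toggle the matching emitter before restarting the system.
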(event Custom|Switch%20Birch
  (bind _leaves (Variables|Default|GetLeaves))
  (Class|NiagaraComponent|SetVariableMaterial _leaves "Leaf_Material" (Variables|Default|GetBirch_Material))
  (Class|NiagaraComponent|SetVariableStaticMesh _leaves "Leaf_Mesh" (Variables|Default|GetBirch_Mesh)))

(event Custom|Switch%20to%20Continuous
  (bind _leaves (Variables|Default|GetLeaves))
  (Variables|Default|SetSwitchedToFloating true)
  (Variables|Default|SetSwitchedToFalling false)
  (Effects|Components|ParticleSystem|SetEmitterEnable (Variables|Default|GetLeaves) "Leaf_Burst" false)
  (Effects|Components|ParticleSystem|SetEmitterEnable (Variables|Default|GetLeaves) "Leaf_SpawnRate" true)
  (Variables|Default|SetSpawn%20Count%20%28Burst%29 0)
  (Niagara|ResetSystem _leaves)
  (Niagara|ReinitializeSystem _leaves))

(event Custom|Switch%20to%20Burst
  (bind _leaves (Variables|Default|GetLeaves))
  (Variables|Default|SetSwitchedToFalling true)
  (Variables|Default|SetSwitchedToFloating false)
  (Effects|Components|ParticleSystem|SetEmitterEnable (Variables|Default|GetLeaves) "Leaf_Burst" true)
  (Effects|Components|ParticleSystem|SetEmitterEnable (Variables|Default|GetLeaves) "Leaf_SpawnRate" false)
  (Variables|Default|SetSpawnRate 0.0)
  (Niagara|ResetSystem _leaves)
  (Niagara|ReinitializeSystem _leaves))

(event Custom|Switch%20to%20Yellow%20Maple
  (bind _leaves (Variables|Default|GetLeaves))
  (Class|NiagaraComponent|SetVariableMaterial _leaves "Leaf_Material" (Variables|Default|GetY_Maple_Material))
  (Class|NiagaraComponent|SetVariableStaticMesh _leaves "Leaf_Mesh" (Variables|Default|GetY_Maple_Mesh)))

(event Custom|Switch%20To%20Maple
  (bind _leaves (Variables|Default|GetLeaves))
  (Class|NiagaraComponent|SetVariableMaterial _leaves "Leaf_Material" (Variables|Default|GetMaple_Material))
  (Class|NiagaraComponent|SetVariableStaticMesh _leaves "Leaf_Mesh" (Variables|Default|GetMaple_Mesh)))

(event Custom|Switch%20to%20Leaf%205
  (bind _leaves (Variables|Default|GetLeaves))
  (Class|NiagaraComponent|SetVariableMaterial _leaves "Leaf_Material" (Variables|Default|GetLeaf5%20Material))
  (Class|NiagaraComponent|SetVariableStaticMesh _leaves "Leaf_Mesh" (Variables|Default|GetBirch_Mesh)))

(event Custom|Switch%20to%20Leaf%204
  (bind _leaves (Variables|Default|GetLeaves))
  (Class|NiagaraComponent|SetVariableMaterial _leaves "Leaf_Material" (Variables|Default|GetLeaf4%20Material))
  (Class|NiagaraComponent|SetVariableStaticMesh _leaves "Leaf_Mesh" (Variables|Default|GetBirch_Mesh)))

(event Custom|Switch%20to%20Leaf%206
  (bind _leaves (Variables|Default|GetLeaves))
  (Class|NiagaraComponent|SetVariableMaterial _leaves "Leaf_Material" (Variables|Default|GetLeaf6%20Material))
  (Class|NiagaraComponent|SetVariableStaticMesh _leaves "Leaf_Mesh" (Variables|Default|GetBirch_Mesh)))

(fn ConstructionScript
  (bind _leaves (Variables|Default|GetLeaves))
  (Utilities|FlowControl|Sequence
    (:then_0
      (Class|NiagaraComponent|SetAsset (Variables|Default|GetLeaves) (Variables|Default|GetNiagara%20System) true)
      (bind _returnvalue (Rendering|Material|CreateDynamicMaterialInstance _leaves 0 "/Game/OnlyLeaves_VFX_Pack/Materials/M_Leaf_Master.M_Leaf_Master" "None" :!class /Script/Engine.PrimitiveComponent))
      (bind _output_get (Variables|Default|SetDMI _returnvalue))
      (Rendering|Material|SetScalarParameterValue _output_get "Color Intensity" (Variables|Default|GetColor%20Intensity) :!class /Script/Engine.MaterialInstanceDynamic))
    (:then_1
      (Niagara|SetNiagaraVariable(Float) _leaves "New float" (Variables|Default|GetSpawnRate))
      (Niagara|SetNiagaraVariable(Float) (Variables|Default|GetLeaves) "Lifetime Min" (Variables|Default|GetLifetime%20Min))
      (Niagara|SetNiagaraVariable(Float) (Variables|Default|GetLeaves) "Lifetime Max" (Variables|Default|GetLifetime%20Max))
      (Effects|Components|ParticleSystem|SetVectorParameter (Variables|Default|GetLeaves) "Wind Speed" (Variables|Default|GetWind%20Speed/Direction))
      (Niagara|SetNiagaraVariable(Float) (Variables|Default|GetLeaves) "SpawnRate" (Variables|Default|GetSpawnRate))
      (Class|NiagaraComponent|SetVariableInt (Variables|Default|GetLeaves) "Spawn Count" (Variables|Default|GetSpawn%20Count%20%28Burst%29))
      (Niagara|SetNiagaraVariable(Float) (Variables|Default|GetLeaves) "Mesh Uniform Scale Min" (/ (Variables|Default|GetMesh%20Scale%20Min) 1e+02))
      (Niagara|SetNiagaraVariable(Float) (Variables|Default|GetLeaves) "Mesh Uniform Scale Max" (/ (Variables|Default|GetMesh%20Scale%20Max) 1e+02))
      (Niagara|SetNiagaraVariable(Vector3) (Variables|Default|GetLeaves) "Cone Axis" (Variables|Default|GetCone%20Axis))
      (Niagara|SetNiagaraVariable(Vector3) (Variables|Default|GetLeaves) "Box Size" (Variables|Default|GetBox%20Location%20Size))
      (Niagara|SetNiagaraVariable(Vector3) (Variables|Default|GetLeaves) "Vortex Axis" (Variables|Default|GetVortex%20Axis))
      (Niagara|SetNiagaraVariable(Float) (Variables|Default|GetLeaves) "Vortex Force Amount" (Variables|Default|GetVortex%20Force%20Amount))
      (Niagara|SetNiagaraVariable(LinearColor) (Variables|Default|GetLeaves) "User.Color" (Variables|Default|GetLeaf%20Shader))
      (Niagara|SetNiagaraVariable(Float) (Variables|Default|GetLeaves) "M_Wind_Intensity" (Variables|Default|GetMaterial%20Wind%20Intensity))
      (Niagara|SetNiagaraVariable(Float) (Variables|Default|GetLeaves) "M_Wind_Speed" (Variables|Default|GetMaterial%20Wind%20Speed)))
    (:then_2
      (switch Utilities|FlowControl|Switch|SwitchonE_Leaf_Selection (Variables|Default|GetSelected%20Leaf)
        (:NewEnumerator0
          (CallFunction|SwitchtoMaple))
        (:NewEnumerator1
          (CallFunction|SwitchBirch))
        (:NewEnumerator2
          (CallFunction|SwitchtoYellowMaple))
        (:NewEnumerator3
          (CallFunction|SwitchtoLeaf4))
        (:NewEnumerator4
          (CallFunction|SwitchtoLeaf5))
        (:NewEnumerator5
          (CallFunction|SwitchtoLeaf6)))
      (switch Utilities|FlowControl|Switch|SwitchonE_Leaf_Behavior (Variables|Default|GetSelect%20Behavior)
        (:NewEnumerator0
          (CallFunction|SwitchtoBurst))
        (:NewEnumerator1
          (CallFunction|SwitchtoContinuous))))))