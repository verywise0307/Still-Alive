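; BP_Mouse is a mouse actor that starts moving when the side-scroller main character touches it while its WindUp value is true.
; On that capsule overlap it makes its WidUp component visible and, through a DoOnce, starts two timelines.
; One timeline adds its track value to the actor's Y location each update without sweeping, while the Spin timeline rolls the Scene component by a fixed step.
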(event OnComponentBeginOverlap(Capsule)
  (params (OverlappedComponent :type Primitive%20Component%20Object%20Reference) (OtherActor :type Actor%20Object%20Reference) (OtherComp :type Primitive%20Component%20Object%20Reference) (OtherBodyIndex :type Integer) (bFromSweep :type Boolean) (SweepResult :type Hit%20Result%20Structure%20%28by%20ref%29))
  (bind _returnvalue (Transformation|GetActorLocation))
  (bind (_x _y _z) (Math|Vector|BreakVector _returnvalue))
  (bind _asbp_super_side_scroller_main_character (Utilities|Casting|CastToBP_SuperSideScroller_MainCharacter OtherActor))
  (if (Variables|/Game/MainCharacter/Blueprints/BP_SuperSideScroller_MainCharacter.BP_SuperSideScroller_MainCharacter_C|GetWindUp _asbp_super_side_scroller_main_character)
    (Rendering|SetVisibility (Variables|Default|GetWidUp) true false)
    (Utilities|FlowControl|DoOnce false
      (:Completed
        (Utilities|FlowControl|Sequence
          (:then_0
            (bind _새_트랙_0 (Timeline|타임라인 Play)
              (:Update
                (Transformation|SetActorLocation (Math|Vector|MakeVector _x (+ _y _새_트랙_0) _z) false false))))
          (:then_1
            (Timeline|Spin Play
              (:Update
                (Transformation|AddLocalRotation (Variables|Default|GetScene) (Math|Rotator|MakeRotator 5.0 0.0 0.0) false false)))))))))

(event EventBeginPlay)

(event EventTick
  (params (DeltaSeconds :type Float%20%28single-precision%29)))

(fn ConstructionScript)