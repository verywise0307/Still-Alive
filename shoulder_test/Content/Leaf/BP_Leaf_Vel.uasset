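; Leaf pile actor that shrinks and puffs maple leaves when the side-scroller player runs through it.
; Box overlap events track whether the main character is inside and keep a reference to it.
; Each tick, while that character moves faster than a speed threshold, LeafBox scales down by a small percentage to a per-axis minimum and a tiny-scaled orange maple Niagara poof spawns at the trigger.
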(event OnComponentBeginOverlap(Box)
  (params (OverlappedComponent :type Primitive%20Component%20Object%20Reference) (OtherActor :type Actor%20Object%20Reference) (OtherComp :type Primitive%20Component%20Object%20Reference) (OtherBodyIndex :type Integer) (bFromSweep :type Boolean) (SweepResult :type Hit%20Result%20Structure%20%28by%20ref%29))
  (bind _asbp_super_side_scroller_main_character (Utilities|Casting|CastToBP_SuperSideScroller_MainCharacter OtherActor))
  (Variables|Default|SetIsPlayerInTrigger true)
  (Variables|Default|SetAs%20BP%20Super%20Side%20Scroller%20Main%20Character_0 _asbp_super_side_scroller_main_character))

(event OnComponentEndOverlap(Box)
  (params (OverlappedComponent :type Primitive%20Component%20Object%20Reference) (OtherActor :type Actor%20Object%20Reference) (OtherComp :type Primitive%20Component%20Object%20Reference) (OtherBodyIndex :type Integer))
  (bind _asbp_super_side_scroller_main_character (Utilities|Casting|CastToBP_SuperSideScroller_MainCharacter OtherActor))
  (Variables|Default|SetIsPlayerInTrigger false))

(event EventBeginPlay)

(event EventTick
  (params (DeltaSeconds :type Float%20%28single-precision%29))
  (bind _as_bp_super_side_scroller_main_character_0 (Variables|Default|GetAs%20BP%20Super%20Side%20Scroller%20Main%20Character_0))
  (bind _leafbox (Variables|Default|GetLeafBox))
  (bind _returnvalue (Transformation|GetWorldScale _leafbox))
  (if (Variables|Default|GetIsPlayerInTrigger)
    (Utilities|IsValid _as_bp_super_side_scroller_main_character_0
      (:Is%20Valid
        (if (> (Math|Vector|VectorLength (Transformation|GetVelocity _as_bp_super_side_scroller_main_character_0)) 4e+02)
          (Transformation|SetWorldScale3D (Variables|Default|GetLeafBox) (Math|Vector|MakeVector (Math|Float|Clamp(Float) (* (.x _returnvalue) 0.99) 0.08) (Math|Float|Clamp(Float) (* (.y _returnvalue) 0.99) 0.02) (Math|Float|Clamp(Float) (* (.z _returnvalue) 0.99) 0.08)))
          (Niagara|SpawnSystematLocation "/Game/asset/OnlyLeaves_VFX_Pack/Niagara/NiagaraLeaves/NS_PoofFloating_OrangeMaple.NS_PoofFloating_OrangeMaple" (Transformation|GetWorldLocation (Variables|Default|GetBox)) "0, 0, 0" "0.000001,0.000001,0.000001"))))))

(fn ConstructionScript)