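; Cat tower actor whose platform swings back and forth along a horizontal arc, with a widget that appears on proximity.
; Each Tick advances or rewinds elapsed time, sets the platform's relative X/Y from sine and cosine scaled by Radius and Speed, and flips direction near either Y extreme.
; Entering the Sphere shows the Widget for up to three seconds, and leaving it hides the Widget immediately.
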(event OnComponentBeginOverlap(Sphere)
  (params (OverlappedComponent :type Primitive%20Component%20Object%20Reference) (OtherActor :type Actor%20Object%20Reference) (OtherComp :type Primitive%20Component%20Object%20Reference) (OtherBodyIndex :type Integer) (bFromSweep :type Boolean) (SweepResult :type Hit%20Result%20Structure%20%28by%20ref%29))
  (bind _widget (Variables|Default|GetWidget))
  (Rendering|SetVisibility _widget true false)
  (Utilities|FlowControl|Delay 3.0)
  (Rendering|SetVisibility _widget false false))

(event OnComponentEndOverlap(Sphere)
  (params (OverlappedComponent :type Primitive%20Component%20Object%20Reference) (OtherActor :type Actor%20Object%20Reference) (OtherComp :type Primitive%20Component%20Object%20Reference) (OtherBodyIndex :type Integer))
  (Rendering|SetVisibility (Variables|Default|GetWidget) false false))

(event EventBeginPlay)

(event Collision|EventActorBeginOverlap
  (params (OtherActor :type Actor%20Object%20Reference)))

(event EventTick
  (params (DeltaSeconds :type Float%20%28single-precision%29))
  (bind _y (|Y_2))
  (bind _y_2 (|Y))
  (Utilities|FlowControl|Sequence
    (:then_1
      (if (Variables|Default|Getclockwise)
        (Variables|Default|Set%20TimeElapsed (+ DeltaSeconds (Variables|Default|Get%20TimeElapsed)))
        (Transformation|SetRelativeLocation (Variables|Default|Getcattowerplatform) (Math|Vector|MakeVector (|X) _y_2 0.0) false false)
        (if (Math|Float|NearlyEqual(Float) _y_2 (Variables|Default|GetRadius) 1.0)
          (Variables|Default|Setclockwise false))
        (else
          (Variables|Default|Set%20TimeElapsed (- (Variables|Default|Get%20TimeElapsed) DeltaSeconds))
          (Transformation|SetRelativeLocation (Variables|Default|Getcattowerplatform) (Math|Vector|MakeVector (|X_2) _y 0.0) false false)
          (if (Math|Float|NearlyEqual(Float) _y (* (Variables|Default|GetRadius) -1.0) 1.0)
            (Variables|Default|Setclockwise true)))))))

(fn ConstructionScript)