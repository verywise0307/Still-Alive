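; BP_cat_tower2 is a cat tower actor that swings back and forth in yaw and shows a widget on overlap.
; Tick turns it at Speed, flipping the Clockwise flag near -1 and -179 degrees for a roughly half-turn sweep.
; Sphere begin overlap shows the Widget component, then hides it after a three-second delay; end overlap hides it immediately.
; A DoOnce gate for the popup is left unconnected.
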(event OnComponentBeginOverlap(Sphere)
  (params (OverlappedComponent :type Primitive%20Component%20Object%20Reference) (OtherActor :type Actor%20Object%20Reference) (OtherComp :type Primitive%20Component%20Object%20Reference) (OtherBodyIndex :type Integer) (bFromSweep :type Boolean) (SweepResult :type Hit%20Result%20Structure%20%28by%20ref%29))
  (bind _widget (Variables|Default|GetWidget))
  (Rendering|SetVisibility _widget true false)
  (Utilities|FlowControl|Delay 3.0)
  (Rendering|SetVisibility _widget false false))

(event OnComponentEndOverlap(Sphere)
  (params (OverlappedComponent :type Primitive%20Component%20Object%20Reference) (OtherActor :type Actor%20Object%20Reference) (OtherComp :type Primitive%20Component%20Object%20Reference) (OtherBodyIndex :type Integer))
  (Rendering|SetVisibility (Variables|Default|GetWidget) false false))

(event EventBeginPlay)

(event Collision|EventActorBeginOverlap
  (params (OtherActor :type Actor%20Object%20Reference)))

(event EventTick
  (params (DeltaSeconds :type Float%20%28single-precision%29))
  (bind _returnvalue (Transformation|GetActorRotation))
  (bind _speed (Variables|Default|Getspeed))
  (bind _returnvalue_2 (* DeltaSeconds _speed))
  (if (Variables|Default|Getclockwise)
    (Transformation|SetActorRotation (Math|Rotator|MakeRotator (.roll _returnvalue) (.pitch _returnvalue) (+ _returnvalue_2 (.yaw _returnvalue))))
    (if (not (<= (.yaw _returnvalue) -1.0))
      (Variables|Default|Setclockwise false))
    (else
      (Transformation|SetActorRotation (Math|Rotator|MakeRotator (.roll _returnvalue) (.pitch _returnvalue) (- (.yaw _returnvalue) _returnvalue_2)))
      (if (not (<= -179.0 (.yaw _returnvalue)))
        (Variables|Default|Setclockwise true)))))

(fn ConstructionScript)