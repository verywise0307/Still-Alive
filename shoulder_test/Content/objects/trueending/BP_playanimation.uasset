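; BP_playanimation is a trigger actor that plays the true ending cutscene and follows it with a dialogue.
; When the main character's MainCapsule overlaps its Box, it disables player input and plays the TrueendingLS level sequence.
; When the sequence finishes, a bound event re-enables input and adds the WBP_TE_Dialogue2 widget to the viewport.
; The overlap has no one-shot guard, and a SetInputModeGameOnly node is left unconnected.
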(event OnComponentBeginOverlap(Box)
  (params (OverlappedComponent :type Primitive%20Component%20Object%20Reference) (OtherActor :type Actor%20Object%20Reference) (OtherComp :type Primitive%20Component%20Object%20Reference) (OtherBodyIndex :type Integer) (bFromSweep :type Boolean) (SweepResult :type Hit%20Result%20Structure%20%28by%20ref%29))
  (bind _asbp_super_side_scroller_main_character (Utilities|Casting|CastToBP_SuperSideScroller_MainCharacter OtherActor))
  (if (== OtherComp (Variables|/Game/MainCharacter/Blueprints/BP_SuperSideScroller_MainCharacter.BP_SuperSideScroller_MainCharacter_C|GetmainCapsule _asbp_super_side_scroller_main_character))
    (Input|DisableInput _asbp_super_side_scroller_main_character (Game|GetPlayerController 0))
    (bind _returnvalue (Sequencer|Player|CreateLevelSequencePlayer "/Game/objects/trueending/trueendingLS.trueendingLS"))
    (Sequencer|Player|Play _returnvalue :!class /Script/MovieScene.MovieSceneSequencePlayer)
    (EventDispatchers|BindEventtoOnFinished _returnvalue (delegate Custom|animend))))

(event Custom|animend
  (Input|EnableInput (stale OnComponentBeginOverlap(Box) _asbp_super_side_scroller_main_character) (Game|GetPlayerController 0))
  (bind _returnvalue (UserInterface|CreateWidget "/Game/objects/trueending/dialoguewVoice/WBP_TE_Dialogue2.WBP_TE_Dialogue2_C" (Game|GetPlayerController 0)))
  (UserInterface|Viewport|AddtoViewport _returnvalue 0))

(event EventBeginPlay)

(event Collision|EventActorBeginOverlap
  (params (OtherActor :type Actor%20Object%20Reference)))

(event EventTick
  (params (DeltaSeconds :type Float%20%28single-precision%29)))

(fn ConstructionScript)