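; A trigger volume for the side-scroller that sets off sprint cats when the player enters its box.
; An overlap by the main character's main capsule plays a 2D meow, waits one second, then searches all BP_sprintcat actors.
; Cats whose Number matches the trigger's own get their Run flag set and RunStart called, and the trigger destroys itself on a match.
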(event OnComponentBeginOverlap(Box)
  (params (OverlappedComponent :type Primitive%20Component%20Object%20Reference) (OtherActor :type Actor%20Object%20Reference) (OtherComp :type Primitive%20Component%20Object%20Reference) (OtherBodyIndex :type Integer) (bFromSweep :type Boolean) (SweepResult :type Hit%20Result%20Structure%20%28by%20ref%29))
  (bind _asbp_super_side_scroller_main_character (Utilities|Casting|CastToBP_SuperSideScroller_MainCharacter OtherActor))
  (if (== (Variables|/Game/MainCharacter/Blueprints/BP_SuperSideScroller_MainCharacter.BP_SuperSideScroller_MainCharacter_C|GetmainCapsule _asbp_super_side_scroller_main_character) OtherComp)
    (Audio|PlaySound2D "/Game/Sound/meow2.meow2" 1.0 1.0 0.0 0 0)
    (Utilities|FlowControl|Delay 1.0)
    (bind _outactors (Actor|GetAllActorsOfClass "/Game/objects/crashcan/BP_sprintcat.BP_sprintcat_C"))
    (for _array_element _outactors
      (if (== (Variables|/Game/objects/crashcan/BP_sprintcat.BP_sprintcat_C|Getnumber _array_element) (Variables|Default|Getnumber))
        (Variables|/Game/objects/crashcan/BP_sprintcat.BP_sprintcat_C|Setrun _array_element true)
        (Default|RunStart _array_element)
        (Actor|DestroyActor)))))

(event EventBeginPlay)

(event Collision|EventActorBeginOverlap
  (params (OtherActor :type Actor%20Object%20Reference)))

(event EventTick
  (params (DeltaSeconds :type Float%20%28single-precision%29)))

(fn ConstructionScript)