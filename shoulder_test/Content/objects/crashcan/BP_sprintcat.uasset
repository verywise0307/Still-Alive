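; BP_sprintcat is a sprinting cat actor that moves along world +Y through its CharacterMovement while its Run flag is true.
; Tick feeds a constant input vector into the movement component; nothing in this graph sets Run.
; The runstart event searches all BP_sprintend actors for a matching Number and stores it as End, which the movement logic does not use.
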(event Custom|run%20start
  (bind _outactors (Actor|GetAllActorsOfClass "/Game/objects/crashcan/BP_sprintend.BP_sprintend_C"))
  (for _array_element _outactors
    (if (== (Variables|/Game/objects/crashcan/BP_sprintend.BP_sprintend_C|Getnumber _array_element) (Variables|Default|Getnumber))
      (Variables|Default|Setend _array_element))))

(event EventBeginPlay)

(event Collision|EventActorBeginOverlap
  (params (OtherActor :type Actor%20Object%20Reference)))

(event EventTick
  (params (DeltaSeconds :type Float%20%28single-precision%29))
  (if (Variables|Default|Getrun)
    (Class|PawnMovementComponent|AddInputVector (Variables|Character|GetCharacterMovement) "0.000000,1.000000,0.000000" false)))

(fn ConstructionScript)