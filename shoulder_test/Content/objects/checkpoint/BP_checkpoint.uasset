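; Checkpoint actor for the side-scroller that saves progress when the player character's main capsule enters its box.
; It loads save slot "1" or creates a new BP_saveobject, then writes the checkpoint's location, current level name, and the player's cat and target catnip counts.
; It also copies those counts into the character's initial-count variables before saving the object back to the slot.
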(event OnComponentBeginOverlap(Box)
  (params (OverlappedComponent :type Primitive%20Component%20Object%20Reference) (OtherActor :type Actor%20Object%20Reference) (OtherComp :type Primitive%20Component%20Object%20Reference) (OtherBodyIndex :type Integer) (bFromSweep :type Boolean) (SweepResult :type Hit%20Result%20Structure%20%28by%20ref%29))
  (bind _returnvalue (Transformation|GetActorLocation))
  (bind _asbp_super_side_scroller_main_character (Utilities|Casting|CastToBP_SuperSideScroller_MainCharacter OtherActor))
  (if (== OtherComp (Variables|/Game/MainCharacter/Blueprints/BP_SuperSideScroller_MainCharacter.BP_SuperSideScroller_MainCharacter_C|GetmainCapsule _asbp_super_side_scroller_main_character))
    (bind _returnvalue_2 (SaveGame|DoesSaveGameExist "1"))
    (if _returnvalue_2
      (bind _returnvalue_3 (SaveGame|LoadGamefromSlot "1"))
      (bind _asbp_saveobject (Utilities|Casting|CastToBP_saveobject _returnvalue_3))
      (Variables|/Game/objects/checkpoint/BP_saveobject.BP_saveobject_C|Setplayer%20position _asbp_saveobject _returnvalue)
      (bind _asbp_super_side_scroller_main_character_2 (Utilities|Casting|CastToBP_SuperSideScroller_MainCharacter (Game|GetPlayerCharacter 0)))
      (Variables|/Game/objects/checkpoint/BP_saveobject.BP_saveobject_C|Setcounttargetcatnip _asbp_saveobject (Variables|/Game/MainCharacter/Blueprints/BP_SuperSideScroller_MainCharacter.BP_SuperSideScroller_MainCharacter_C|Gettargetcatnip _asbp_super_side_scroller_main_character_2))
      (Variables|/Game/objects/checkpoint/BP_saveobject.BP_saveobject_C|Setcountcat _asbp_saveobject (Variables|/Game/MainCharacter/Blueprints/BP_SuperSideScroller_MainCharacter.BP_SuperSideScroller_MainCharacter_C|Getcountcat _asbp_super_side_scroller_main_character_2))
      (Variables|/Game/MainCharacter/Blueprints/BP_SuperSideScroller_MainCharacter.BP_SuperSideScroller_MainCharacter_C|Setinitcountcat _asbp_super_side_scroller_main_character_2 (Variables|/Game/MainCharacter/Blueprints/BP_SuperSideScroller_MainCharacter.BP_SuperSideScroller_MainCharacter_C|Getcountcat _asbp_super_side_scroller_main_character_2))
      (Variables|/Game/MainCharacter/Blueprints/BP_SuperSideScroller_MainCharacter.BP_SuperSideScroller_MainCharacter_C|Setinitcounttargetcatnip _asbp_super_side_scroller_main_character_2 (Variables|/Game/MainCharacter/Blueprints/BP_SuperSideScroller_MainCharacter.BP_SuperSideScroller_MainCharacter_C|Gettargetcatnip _asbp_super_side_scroller_main_character_2))
      (bind _returnvalue_4 (Game|GetCurrentLevelName true))
      (Variables|/Game/objects/checkpoint/BP_saveobject.BP_saveobject_C|Setcurmapname _asbp_saveobject _returnvalue_4)
      (SaveGame|SaveGametoSlot _asbp_saveobject "1")
      (else
        (bind _returnvalue_5 (SaveGame|CreateSaveGameObject "/Game/objects/checkpoint/BP_saveobject.BP_saveobject_C"))
        (Variables|/Game/objects/checkpoint/BP_saveobject.BP_saveobject_C|Setplayer%20position _returnvalue_5 _returnvalue)
        (bind _asbp_super_side_scroller_main_character_3 (Utilities|Casting|CastToBP_SuperSideScroller_MainCharacter (Game|GetPlayerCharacter 0)))
        (Variables|/Game/objects/checkpoint/BP_saveobject.BP_saveobject_C|Setcounttargetcatnip _returnvalue_5 (Variables|/Game/MainCharacter/Blueprints/BP_SuperSideScroller_MainCharacter.BP_SuperSideScroller_MainCharacter_C|Gettargetcatnip _asbp_super_side_scroller_main_character_3))
        (Variables|/Game/objects/checkpoint/BP_saveobject.BP_saveobject_C|Setcountcat _returnvalue_5 (Variables|/Game/MainCharacter/Blueprints/BP_SuperSideScroller_MainCharacter.BP_SuperSideScroller_MainCharacter_C|Getcountcat _asbp_super_side_scroller_main_character_3))
        (Variables|/Game/MainCharacter/Blueprints/BP_SuperSideScroller_MainCharacter.BP_SuperSideScroller_MainCharacter_C|Setinitcountcat _asbp_super_side_scroller_main_character_3 (Variables|/Game/MainCharacter/Blueprints/BP_SuperSideScroller_MainCharacter.BP_SuperSideScroller_MainCharacter_C|Getcountcat _asbp_super_side_scroller_main_character_3))
        (Variables|/Game/MainCharacter/Blueprints/BP_SuperSideScroller_MainCharacter.BP_SuperSideScroller_MainCharacter_C|Setinitcounttargetcatnip _asbp_super_side_scroller_main_character_3 (Variables|/Game/MainCharacter/Blueprints/BP_SuperSideScroller_MainCharacter.BP_SuperSideScroller_MainCharacter_C|Gettargetcatnip _asbp_super_side_scroller_main_character_3))
        (bind _returnvalue_6 (Game|GetCurrentLevelName true))
        (Variables|/Game/objects/checkpoint/BP_saveobject.BP_saveobject_C|Setcurmapname _returnvalue_5 _returnvalue_6)
        (SaveGame|SaveGametoSlot _returnvalue_5 "1")))))

(event EventBeginPlay)

(event Collision|EventActorBeginOverlap
  (params (OtherActor :type Actor%20Object%20Reference)))

(event EventTick
  (params (DeltaSeconds :type Float%20%28single-precision%29)))

(fn ConstructionScript)