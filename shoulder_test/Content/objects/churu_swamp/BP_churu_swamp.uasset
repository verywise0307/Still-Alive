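; BP_churu_swamp is a swamp actor whose ground gradually gives way while the player is in it.
; Begin and end overlap on Playeroverlap set Isplayerinswamp, responding only to the BP_ThirdPersonCharacter's mesh.
; Each Tick, AddLocalTransform slowly shrinks the Groundcollision Z scale toward zero while occupied and grows it back much faster to about its cap when empty.
; The scale changes are fixed per-frame steps, so their speed depends on frame rate.
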(event OnComponentBeginOverlap(playeroverlap)
  (params (OverlappedComponent :type Primitive%20Component%20Object%20Reference) (OtherActor :type Actor%20Object%20Reference) (OtherComp :type Primitive%20Component%20Object%20Reference) (OtherBodyIndex :type Integer) (bFromSweep :type Boolean) (SweepResult :type Hit%20Result%20Structure%20%28by%20ref%29))
  (bind _asbp_third_person_character (Utilities|Casting|CastToBP_ThirdPersonCharacter OtherActor))
  (if (== OtherComp (Variables|/Script/Engine.Character|GetMesh _asbp_third_person_character))
    (Variables|Default|Setisplayerinswamp true)))

(event OnComponentEndOverlap(playeroverlap)
  (params (OverlappedComponent :type Primitive%20Component%20Object%20Reference) (OtherActor :type Actor%20Object%20Reference) (OtherComp :type Primitive%20Component%20Object%20Reference) (OtherBodyIndex :type Integer))
  (bind _asbp_third_person_character (Utilities|Casting|CastToBP_ThirdPersonCharacter OtherActor))
  (if (== OtherComp (Variables|/Script/Engine.Character|GetMesh _asbp_third_person_character))
    (Variables|Default|Setisplayerinswamp false)))

(event EventBeginPlay)

(event Collision|EventActorBeginOverlap
  (params (OtherActor :type Actor%20Object%20Reference)))

(event EventTick
  (params (DeltaSeconds :type Float%20%28single-precision%29))
  (bind _groundcollision (Variables|Default|Getgroundcollision))
  (bind _returnvalue (Transformation|GetWorldScale _groundcollision))
  (if (Variables|Default|Getisplayerinswamp)
    (if (> (.z _returnvalue) 0.0)
      (Class|SceneComponent|AddLocalTransform _groundcollision (Math|Transform|MakeTransform "0, 0, 0" "0, 0, 0" (Math|Vector|MakeVector (.x _returnvalue) (.y _returnvalue) (- (.z _returnvalue) 0.002))) false false))
    (elif (<= (.z _returnvalue) 1.6)
      (Class|SceneComponent|AddLocalTransform _groundcollision (Math|Transform|MakeTransform "0, 0, 0" "0, 0, 0" (Math|Vector|MakeVector (.x _returnvalue) (.y _returnvalue) (+ (.z _returnvalue) 0.05))) false false))))

(fn ConstructionScript)