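; BP_Launchpad is a launch pad actor that bounces the side-scroller player character upward.
; When its Box is overlapped by the Foot component of BP_SuperSideScroller_MainCharacter, it zeroes the character's vertical velocity, keeping horizontal motion, then calls LaunchCharacter with a fixed upward velocity.
; An earlier attempt to compensate using capsule physics velocity is left disconnected and never runs.
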(event OnComponentBeginOverlap(Box)
  (params (OverlappedComponent :type Primitive%20Component%20Object%20Reference) (OtherActor :type Actor%20Object%20Reference) (OtherComp :type Primitive%20Component%20Object%20Reference) (OtherBodyIndex :type Integer) (bFromSweep :type Boolean) (SweepResult :type Hit%20Result%20Structure%20%28by%20ref%29))
  (bind _asbp_super_side_scroller_main_character (Utilities|Casting|CastToBP_SuperSideScroller_MainCharacter OtherActor))
  (if (== OtherComp (Variables|/Game/MainCharacter/Blueprints/BP_SuperSideScroller_MainCharacter.BP_SuperSideScroller_MainCharacter_C|Getfoot _asbp_super_side_scroller_main_character))
    (Variables|/Script/Engine.MovementComponent|SetVelocity (Variables|/Script/Engine.Character|GetCharacterMovement _asbp_super_side_scroller_main_character) (Math|Vector|MakeVector (.x (Variables|/Script/Engine.MovementComponent|GetVelocity (Variables|/Script/Engine.Character|GetCharacterMovement _asbp_super_side_scroller_main_character))) (.y (Variables|/Script/Engine.MovementComponent|GetVelocity (Variables|/Script/Engine.Character|GetCharacterMovement _asbp_super_side_scroller_main_character))) 0.0))
    (Character|LaunchCharacter _asbp_super_side_scroller_main_character (Math|Vector|MakeVector 0.0 0.0 1.5e+03) false false)))

(event EventBeginPlay)

(event Collision|EventActorBeginOverlap
  (params (OtherActor :type Actor%20Object%20Reference)))

(event EventTick
  (params (DeltaSeconds :type Float%20%28single-precision%29)))

(fn ConstructionScript)