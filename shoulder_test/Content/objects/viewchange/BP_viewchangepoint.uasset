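; BP_viewchangepoint is a trigger volume marking a spot where the side-scroller main character is allowed to change view.
; When the character's MainCapsule begins overlapping the Box, it sets the character's Canchangeview flag and passes the actor's location as Viewchangepoint.
; When that capsule leaves, it clears the flag but keeps the stored point; the view switch itself is not handled here.
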(event OnComponentBeginOverlap(Box)
  (params (OverlappedComponent :type Primitive%20Component%20Object%20Reference) (OtherActor :type Actor%20Object%20Reference) (OtherComp :type Primitive%20Component%20Object%20Reference) (OtherBodyIndex :type Integer) (bFromSweep :type Boolean) (SweepResult :type Hit%20Result%20Structure%20%28by%20ref%29))
  (bind _asbp_super_side_scroller_main_character (Utilities|Casting|CastToBP_SuperSideScroller_MainCharacter OtherActor))
  (if (== (Variables|/Game/MainCharacter/Blueprints/BP_SuperSideScroller_MainCharacter.BP_SuperSideScroller_MainCharacter_C|GetmainCapsule _asbp_super_side_scroller_main_character) OtherComp)
    (Variables|/Game/MainCharacter/Blueprints/BP_SuperSideScroller_MainCharacter.BP_SuperSideScroller_MainCharacter_C|SetCanchangeview _asbp_super_side_scroller_main_character true)
    (Variables|/Game/MainCharacter/Blueprints/BP_SuperSideScroller_MainCharacter.BP_SuperSideScroller_MainCharacter_C|Setviewchangepoint _asbp_super_side_scroller_main_character (Transformation|GetActorLocation))))

(event OnComponentEndOverlap(Box)
  (params (OverlappedComponent :type Primitive%20Component%20Object%20Reference) (OtherActor :type Actor%20Object%20Reference) (OtherComp :type Primitive%20Component%20Object%20Reference) (OtherBodyIndex :type Integer))
  (bind _asbp_super_side_scroller_main_character (Utilities|Casting|CastToBP_SuperSideScroller_MainCharacter OtherActor))
  (if (== (Variables|/Game/MainCharacter/Blueprints/BP_SuperSideScroller_MainCharacter.BP_SuperSideScroller_MainCharacter_C|GetmainCapsule _asbp_super_side_scroller_main_character) OtherComp)
    (Variables|/Game/MainCharacter/Blueprints/BP_SuperSideScroller_MainCharacter.BP_SuperSideScroller_MainCharacter_C|Setcanchangeview _asbp_super_side_scroller_main_character false)))

(event EventBeginPlay)

(event Collision|EventActorBeginOverlap
  (params (OtherActor :type Actor%20Object%20Reference)))

(event EventTick
  (params (DeltaSeconds :type Float%20%28single-precision%29)))

(fn ConstructionScript)