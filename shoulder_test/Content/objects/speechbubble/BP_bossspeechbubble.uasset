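; Boss speech bubble trigger that shows a line of text on screen once, when the side-scroller main character's main capsule enters its box.
; BeginPlay creates the WB_bossspeechbubble widget, fills it from the String variable with "\n" removed, and assigns it to the hidden Speechbubble component.
; The overlap adds that widget to the viewport, removes it after a short delay, then destroys the actor.
; Player-follow and component-visibility nodes are disconnected, leaving Tick without effect.
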(event OnComponentBeginOverlap(Box)
  (params (OverlappedComponent :type Primitive%20Component%20Object%20Reference) (OtherActor :type Actor%20Object%20Reference) (OtherComp :type Primitive%20Component%20Object%20Reference) (OtherBodyIndex :type Integer) (bFromSweep :type Boolean) (SweepResult :type Hit%20Result%20Structure%20%28by%20ref%29))
  (bind _wb (Variables|Default|GetWB))
  (bind _asbp_super_side_scroller_main_character (Utilities|Casting|CastToBP_SuperSideScroller_MainCharacter OtherActor))
  (if (== OtherComp (Variables|/Game/MainCharacter/Blueprints/BP_SuperSideScroller_MainCharacter.BP_SuperSideScroller_MainCharacter_C|GetmainCapsule _asbp_super_side_scroller_main_character))
    (Utilities|FlowControl|DoOnce false
      (:Completed
        (Variables|Default|Setplayeroverlap true)
        (UserInterface|Viewport|AddtoViewport _wb 0)
        (Utilities|FlowControl|Delay 3.0)
        (Widget|RemovefromParent _wb)
        (Actor|DestroyActor)))))

(event EventBeginPlay
  (Rendering|SetVisibility (Variables|Default|Getspeechbubble) false false)
  (bind _returnvalue (UserInterface|CreateWidget "/Game/UI/Meowment/WB_bossspeechbubble.WB_bossspeechbubble_C"))
  (bind _output_get (Variables|Default|Setwb _returnvalue))
  (Variables|/Game/UI/Meowment/WB_bossspeechbubble.WB_bossspeechbubble_C|Setstring _output_get (Utilities|Text|ToText(String) (Utilities|String|Replace (Variables|Default|Getstring) "\\n" " 
")))
  (UserInterface|SetWidget (Variables|Default|Getspeechbubble) (Variables|Default|GetWB)))

(event Collision|EventActorBeginOverlap
  (params (OtherActor :type Actor%20Object%20Reference)))

(event EventTick
  (params (DeltaSeconds :type Float%20%28single-precision%29))
  (if (Variables|Default|Getplayeroverlap)
    _))

(fn ConstructionScript)