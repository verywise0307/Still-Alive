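; BP_sign is a readable sign for the side-scroller that displays a WB_sign screen widget with its Image texture.
; Sphere overlap tracks the player's main capsule; Tick adds the widget while the player is inside and the character's Sign flag is true, otherwise removes it.
; The first Box overlap by any actor shows a separate Widget component for three seconds, hiding it early on end overlap.
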(event OnComponentBeginOverlap(Sphere)
  (params (OverlappedComponent :type Primitive%20Component%20Object%20Reference) (OtherActor :type Actor%20Object%20Reference) (OtherComp :type Primitive%20Component%20Object%20Reference) (OtherBodyIndex :type Integer) (bFromSweep :type Boolean) (SweepResult :type Hit%20Result%20Structure%20%28by%20ref%29))
  (bind _asbp_super_side_scroller_main_character (Utilities|Casting|CastToBP_SuperSideScroller_MainCharacter OtherActor))
  (if (== (Variables|/Game/MainCharacter/Blueprints/BP_SuperSideScroller_MainCharacter.BP_SuperSideScroller_MainCharacter_C|GetmainCapsule _asbp_super_side_scroller_main_character) OtherComp)
    (Variables|Default|Setplayer%20overlap true)))

(event OnComponentEndOverlap(Sphere)
  (params (OverlappedComponent :type Primitive%20Component%20Object%20Reference) (OtherActor :type Actor%20Object%20Reference) (OtherComp :type Primitive%20Component%20Object%20Reference) (OtherBodyIndex :type Integer))
  (bind _asbp_super_side_scroller_main_character (Utilities|Casting|CastToBP_SuperSideScroller_MainCharacter OtherActor))
  (if (== (Variables|/Game/MainCharacter/Blueprints/BP_SuperSideScroller_MainCharacter.BP_SuperSideScroller_MainCharacter_C|GetmainCapsule _asbp_super_side_scroller_main_character) OtherComp)
    (Widget|RemovefromParent (Variables|Default|Getwb))
    (Variables|Default|Setadd false)
    (Variables|Default|Setplayer%20overlap false)))

(event OnComponentBeginOverlap(Box)
  (params (OverlappedComponent :type Primitive%20Component%20Object%20Reference) (OtherActor :type Actor%20Object%20Reference) (OtherComp :type Primitive%20Component%20Object%20Reference) (OtherBodyIndex :type Integer) (bFromSweep :type Boolean) (SweepResult :type Hit%20Result%20Structure%20%28by%20ref%29))
  (bind _widget (Variables|Default|GetWidget))
  (Utilities|FlowControl|DoOnce false
    (:Completed
      (Rendering|SetVisibility _widget true false)
      (Utilities|FlowControl|Delay 3.0)
      (Rendering|SetVisibility _widget false false))))

(event OnComponentEndOverlap(Box)
  (params (OverlappedComponent :type Primitive%20Component%20Object%20Reference) (OtherActor :type Actor%20Object%20Reference) (OtherComp :type Primitive%20Component%20Object%20Reference) (OtherBodyIndex :type Integer))
  (Rendering|SetVisibility (Variables|Default|GetWidget) false false))

(event EventBeginPlay
  (bind _returnvalue (UserInterface|CreateWidget "/Game/objects/sign/WB_sign.WB_sign_C"))
  (bind _output_get (Variables|Default|Setwb _returnvalue))
  (Appearance|SetBrushfromTexture (Variables|/Game/objects/sign/WB_sign.WB_sign_C|GetImage_51 _output_get) (Variables|Default|Getimage) false))

(event Collision|EventActorBeginOverlap
  (params (OtherActor :type Actor%20Object%20Reference)))

(event EventTick
  (params (DeltaSeconds :type Float%20%28single-precision%29))
  (bind _asbp_super_side_scroller_main_character (Utilities|Casting|CastToBP_SuperSideScroller_MainCharacter (Game|GetPlayerCharacter 0)))
  (if (Math|Boolean|ANDBoolean (Variables|/Game/MainCharacter/Blueprints/BP_SuperSideScroller_MainCharacter.BP_SuperSideScroller_MainCharacter_C|Getsign _asbp_super_side_scroller_main_character) (Variables|Default|Getplayer%20overlap) (not (Variables|Default|Getadd)))
    (UserInterface|Viewport|AddtoViewport (Variables|Default|Getwb) 0)
    (else
      (Widget|RemovefromParent (Variables|Default|Getwb))
      (Variables|Default|Setadd false))))

(fn ConstructionScript)