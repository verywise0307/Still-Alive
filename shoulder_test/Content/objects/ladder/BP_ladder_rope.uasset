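; Climbable rope ladder for the side-scroller main character, with a pressure-switch counter.
; Box overlap with the character's LadderBox enables climbing, and leaving clears the climb state and restores gravity and walking.
; While the player is on the ladder without horizontal input, Tick snaps them to the ladder's Y and zeroes rotation.
; Switchactive counts activations to play or reverse a timeline, but the location update using its track is unwired.
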(event OnComponentBeginOverlap(Box)
  (params (OverlappedComponent :type Primitive%20Component%20Object%20Reference) (OtherActor :type Actor%20Object%20Reference) (OtherComp :type Primitive%20Component%20Object%20Reference) (OtherBodyIndex :type Integer) (bFromSweep :type Boolean) (SweepResult :type Hit%20Result%20Structure%20%28by%20ref%29))
  (bind _asbp_super_side_scroller_main_character (Utilities|Casting|CastToBP_SuperSideScroller_MainCharacter OtherActor))
  (if (== (Variables|/Game/MainCharacter/Blueprints/BP_SuperSideScroller_MainCharacter.BP_SuperSideScroller_MainCharacter_C|Getladder%20box _asbp_super_side_scroller_main_character) OtherComp)
    (Variables|/Script/shoulder_test.shoulder_testCharacter|Setcanclimb _asbp_super_side_scroller_main_character true)
    (Variables|Default|Setplayeroverlap true)))

(event OnComponentEndOverlap(Box)
  (params (OverlappedComponent :type Primitive%20Component%20Object%20Reference) (OtherActor :type Actor%20Object%20Reference) (OtherComp :type Primitive%20Component%20Object%20Reference) (OtherBodyIndex :type Integer))
  (bind _asbp_super_side_scroller_main_character (Utilities|Casting|CastToBP_SuperSideScroller_MainCharacter OtherActor))
  (if (== (Variables|/Game/MainCharacter/Blueprints/BP_SuperSideScroller_MainCharacter.BP_SuperSideScroller_MainCharacter_C|Getladder%20box _asbp_super_side_scroller_main_character) OtherComp)
    (Variables|/Script/shoulder_test.shoulder_testCharacter|Setcanclimb _asbp_super_side_scroller_main_character false)
    (Variables|/Game/MainCharacter/Blueprints/BP_SuperSideScroller_MainCharacter.BP_SuperSideScroller_MainCharacter_C|Setisonladder _asbp_super_side_scroller_main_character false)
    (Variables|Default|Setplayeroverlap false)
    (Variables|/Script/Engine.CharacterMovementComponent|SetGravityScale (Variables|/Script/Engine.Character|GetCharacterMovement _asbp_super_side_scroller_main_character) 2.25)
    (Pawn|Components|CharacterMovement|SetMovementMode (Variables|/Script/Engine.Character|GetCharacterMovement _asbp_super_side_scroller_main_character) "MOVE_Walking" 0)))

(event Custom|Switchactive
  (Math|Integer|IncrementInt (Variables|Default|Getpressureactive)
    (:%20%20
      (if (>= (Variables|Default|Getpressureactive) (Variables|Default|Getpressureneeded))
        (bind _새_트랙_0 (Timeline|타임라인 Play))
        (else
          (Timeline|타임라인 Reverse))))))

(event EventTick
  (params (DeltaSeconds :type Float%20%28single-precision%29))
  (bind _asbp_super_side_scroller_main_character (Utilities|Casting|CastToBP_SuperSideScroller_MainCharacter (Game|Player|GetPlayerPawn 0)))
  (if (and (Variables|/Game/MainCharacter/Blueprints/BP_SuperSideScroller_MainCharacter.BP_SuperSideScroller_MainCharacter_C|Getisonladder _asbp_super_side_scroller_main_character) (Variables|Default|Getplayeroverlap))
    (if (== (Variables|/Game/MainCharacter/Blueprints/BP_SuperSideScroller_MainCharacter.BP_SuperSideScroller_MainCharacter_C|Getmove%20right _asbp_super_side_scroller_main_character) 0.0)
      (Transformation|SetActorLocationAndRotation _asbp_super_side_scroller_main_character (Math|Vector|MakeVector (.x (Transformation|GetActorLocation _asbp_super_side_scroller_main_character)) (.y (Transformation|GetActorLocation)) (.z (Transformation|GetActorLocation _asbp_super_side_scroller_main_character))) "0.000000,0.000000,0.000000"))))

(fn ConstructionScript)