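; A climbable moving ladder for the side-scroller main character.
; Its Box overlap with the character's LadderBox toggles climbing, restoring walking and gravity on exit.
; While the player is on it, Tick compares the ladder's Z to its previous position and nudges the character up or down at a fixed rate to follow it.
; The Capsule reveals a widget once, hiding it after a delay or on exit.
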(event OnComponentBeginOverlap(Box)
  (params (OverlappedComponent :type Primitive%20Component%20Object%20Reference) (OtherActor :type Actor%20Object%20Reference) (OtherComp :type Primitive%20Component%20Object%20Reference) (OtherBodyIndex :type Integer) (bFromSweep :type Boolean) (SweepResult :type Hit%20Result%20Structure%20%28by%20ref%29))
  (bind _asbp_super_side_scroller_main_character (Utilities|Casting|CastToBP_SuperSideScroller_MainCharacter OtherActor))
  (if (== (Variables|/Game/MainCharacter/Blueprints/BP_SuperSideScroller_MainCharacter.BP_SuperSideScroller_MainCharacter_C|Getladder%20box _asbp_super_side_scroller_main_character) OtherComp)
    (Variables|/Script/shoulder_test.shoulder_testCharacter|Setcanclimb _asbp_super_side_scroller_main_character true)
    (Variables|Default|Setplayeroverlap true)))

(event OnComponentEndOverlap(Box)
  (params (OverlappedComponent :type Primitive%20Component%20Object%20Reference) (OtherActor :type Actor%20Object%20Reference) (OtherComp :type Primitive%20Component%20Object%20Reference) (OtherBodyIndex :type Integer))
  (bind _asbp_super_side_scroller_main_character (Utilities|Casting|CastToBP_SuperSideScroller_MainCharacter OtherActor))
  (if (== (Variables|/Game/MainCharacter/Blueprints/BP_SuperSideScroller_MainCharacter.BP_SuperSideScroller_MainCharacter_C|Getladder%20box _asbp_super_side_scroller_main_character) OtherComp)
    (Variables|/Script/shoulder_test.shoulder_testCharacter|Setcanclimb _asbp_super_side_scroller_main_character false)
    (Variables|/Game/MainCharacter/Blueprints/BP_SuperSideScroller_MainCharacter.BP_SuperSideScroller_MainCharacter_C|Setisonladder _asbp_super_side_scroller_main_character false)
    (Variables|/Script/Engine.CharacterMovementComponent|SetGravityScale (Variables|/Script/Engine.Character|GetCharacterMovement _asbp_super_side_scroller_main_character) 2.25)
    (Pawn|Components|CharacterMovement|SetMovementMode (Variables|/Script/Engine.Character|GetCharacterMovement _asbp_super_side_scroller_main_character) "MOVE_Walking" 0)
    (Variables|Default|Setplayeroverlap false)))

(event OnComponentBeginOverlap(Capsule)
  (params (OverlappedComponent :type Primitive%20Component%20Object%20Reference) (OtherActor :type Actor%20Object%20Reference) (OtherComp :type Primitive%20Component%20Object%20Reference) (OtherBodyIndex :type Integer) (bFromSweep :type Boolean) (SweepResult :type Hit%20Result%20Structure%20%28by%20ref%29))
  (bind _widget (Variables|Default|GetWidget))
  (Utilities|FlowControl|DoOnce false
    (:Completed
      (Rendering|SetVisibility _widget true false)
      (Utilities|FlowControl|Delay 3.0)
      (Rendering|SetVisibility _widget false false))))

(event OnComponentEndOverlap(Capsule)
  (params (OverlappedComponent :type Primitive%20Component%20Object%20Reference) (OtherActor :type Actor%20Object%20Reference) (OtherComp :type Primitive%20Component%20Object%20Reference) (OtherBodyIndex :type Integer))
  (Rendering|SetVisibility (Variables|Default|GetWidget) false false))

(event EventTick
  (params (DeltaSeconds :type Float%20%28single-precision%29))
  (bind _returnvalue (Transformation|GetActorLocation))
  (bind _returnvalue_2 (* 75.0 DeltaSeconds))
  (bind _asbp_super_side_scroller_main_character (Utilities|Casting|CastToBP_SuperSideScroller_MainCharacter (Game|GetPlayerCharacter 0)))
  (if (and (Variables|/Game/MainCharacter/Blueprints/BP_SuperSideScroller_MainCharacter.BP_SuperSideScroller_MainCharacter_C|Getisonladder _asbp_super_side_scroller_main_character) (Variables|Default|Getplayeroverlap))
    (if (< (.z (Variables|Default|Getprevious%20location)) (.z (Transformation|GetActorLocation)))
      (Variables|Default|Setprevious%20location _returnvalue)
      (Transformation|AddActorWorldOffset _asbp_super_side_scroller_main_character (Math|Vector|MakeVector 0.0 0.0 _returnvalue_2))
      (else
        (Variables|Default|Setprevious%20location _returnvalue)
        (Transformation|AddActorWorldOffset _asbp_super_side_scroller_main_character (Math|Vector|MakeVector 0.0 0.0 (* _returnvalue_2 -1.0)))))))

(event EventBeginPlay)

(fn ConstructionScript)