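; BP_targetcatnip is a catnip collectible for the side-scroller that stays collected through a per-index flag in GI_stage.
; On BeginPlay it destroys itself if already flagged.
; When its sphere overlaps the player's main capsule, it increments character and game instance counters and sets the flag.
; If save slot 1 exists, it saves the count, shows a dialogue widget on the fifth pickup, and destroys itself.
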(event OnComponentBeginOverlap(Sphere)
  (params (OverlappedComponent :type Primitive%20Component%20Object%20Reference) (OtherActor :type Actor%20Object%20Reference) (OtherComp :type Primitive%20Component%20Object%20Reference) (OtherBodyIndex :type Integer) (bFromSweep :type Boolean) (SweepResult :type Hit%20Result%20Structure%20%28by%20ref%29))
  (bind _asbp_super_side_scroller_main_character (Utilities|Casting|CastToBP_SuperSideScroller_MainCharacter OtherActor))
  (if (== OtherComp (Variables|/Game/MainCharacter/Blueprints/BP_SuperSideScroller_MainCharacter.BP_SuperSideScroller_MainCharacter_C|GetmainCapsule _asbp_super_side_scroller_main_character))
    (bind _result (Math|Integer|IncrementInt (Variables|/Game/MainCharacter/Blueprints/BP_SuperSideScroller_MainCharacter.BP_SuperSideScroller_MainCharacter_C|Gettargetcatnip _asbp_super_side_scroller_main_character))
      (:%20%20
        (bind _asgi_stage (Utilities|Casting|CastToGI_stage (Game|GetGameInstance)))
        (Math|Integer|IncrementInt (Variables|/Game/MainCharacter/Blueprints/GI_stage.GI_stage_C|Getitem3 _asgi_stage)
          (:%20%20
            (Math|Integer|IncrementInt (Variables|/Game/MainCharacter/Blueprints/GI_stage.GI_stage_C|Getitem _asgi_stage)
              (:%20%20
                (Utilities|Array|SetArrayElem (Variables|/Game/MainCharacter/Blueprints/GI_stage.GI_stage_C|Getcatnip _asgi_stage) (Variables|Default|Getnum) true)
                (bind _returnvalue (SaveGame|DoesSaveGameExist "1"))
                (if _returnvalue
                  (bind _returnvalue_2 (SaveGame|LoadGamefromSlot "1"))
                  (bind _asbp_saveobject (Utilities|Casting|CastToBP_saveobject _returnvalue_2))
                  (bind _asbp_super_side_scroller_main_character_2 (Utilities|Casting|CastToBP_SuperSideScroller_MainCharacter (Game|GetPlayerCharacter 0)))
                  (bind _output_get (Variables|/Game/objects/checkpoint/BP_saveobject.BP_saveobject_C|Setcounttargetcatnip _asbp_saveobject _result))
                  (Variables|/Game/MainCharacter/Blueprints/BP_SuperSideScroller_MainCharacter.BP_SuperSideScroller_MainCharacter_C|Setinitcounttargetcatnip _asbp_super_side_scroller_main_character_2 _output_get)
                  (SaveGame|SaveGametoSlot _asbp_saveobject "1")
                  (if (== _result 5)
                    (bind _returnvalue_3 (UserInterface|CreateWidget "/Game/objects/cats/Dialogue_wSound/WBP_catnipDialogue_1.WBP_catnipDialogue_1_C"))
                    (UserInterface|Viewport|AddtoViewport _returnvalue_3 0)
                    (Variables|/Game/MainCharacter/Blueprints/GI_stage.GI_stage_C|Set5catnip _asgi_stage true))
                  (Actor|DestroyActor))))))))))

(event EventBeginPlay
  (bind _asgi_stage (Utilities|Casting|CastToGI_stage (Game|GetGameInstance)))
  (if (Utilities|Array|Get(acopy) (Variables|/Game/MainCharacter/Blueprints/GI_stage.GI_stage_C|Getcatnip _asgi_stage) (Variables|Default|Getnum))
    (Actor|DestroyActor)))

(event Collision|EventActorBeginOverlap
  (params (OtherActor :type Actor%20Object%20Reference)))

(event EventTick
  (params (DeltaSeconds :type Float%20%28single-precision%29)))

(fn ConstructionScript)