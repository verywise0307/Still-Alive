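; Stage 3 cat NPC that opens a dialogue for the side-scroller player and switches to a lying caress animation once Stage3cat1 is set.
; Tick polls the player's Sign flag and Sphere overlap, then logs the chat and creates WBP_catDialogue1.
; Npcchatlog increments GI_stage counters by level name, with Stage3_2 sharing Npcchat2 with Stage 2.
; A Box overlap briefly shows a widget once, hiding it after a delay or on exit.
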(event OnComponentBeginOverlap(Sphere)
  (params (OverlappedComponent :type Primitive%20Component%20Object%20Reference) (OtherActor :type Actor%20Object%20Reference) (OtherComp :type Primitive%20Component%20Object%20Reference) (OtherBodyIndex :type Integer) (bFromSweep :type Boolean) (SweepResult :type Hit%20Result%20Structure%20%28by%20ref%29))
  (bind _asbp_super_side_scroller_main_character (Utilities|Casting|CastToBP_SuperSideScroller_MainCharacter OtherActor))
  (if (== OtherComp (Variables|/Game/MainCharacter/Blueprints/BP_SuperSideScroller_MainCharacter.BP_SuperSideScroller_MainCharacter_C|GetmainCapsule _asbp_super_side_scroller_main_character))
    (Variables|Default|Setplayer%20overlap true)))

(event OnComponentEndOverlap(Sphere)
  (params (OverlappedComponent :type Primitive%20Component%20Object%20Reference) (OtherActor :type Actor%20Object%20Reference) (OtherComp :type Primitive%20Component%20Object%20Reference) (OtherBodyIndex :type Integer))
  (bind _asbp_super_side_scroller_main_character (Utilities|Casting|CastToBP_SuperSideScroller_MainCharacter OtherActor))
  (if (== OtherComp (Variables|/Game/MainCharacter/Blueprints/BP_SuperSideScroller_MainCharacter.BP_SuperSideScroller_MainCharacter_C|GetmainCapsule _asbp_super_side_scroller_main_character))
    (Variables|Default|Setplayer%20overlap false)))

(event OnComponentBeginOverlap(Box)
  (params (OverlappedComponent :type Primitive%20Component%20Object%20Reference) (OtherActor :type Actor%20Object%20Reference) (OtherComp :type Primitive%20Component%20Object%20Reference) (OtherBodyIndex :type Integer) (bFromSweep :type Boolean) (SweepResult :type Hit%20Result%20Structure%20%28by%20ref%29))
  (bind _widget (Variables|Default|GetWidget))
  (Utilities|FlowControl|DoOnce false
    (:Completed
      (Rendering|SetVisibility _widget true false)
      (Utilities|FlowControl|Delay 1.0)
      (Rendering|SetVisibility _widget false false))))

(event OnComponentEndOverlap(Box)
  (params (OverlappedComponent :type Primitive%20Component%20Object%20Reference) (OtherActor :type Actor%20Object%20Reference) (OtherComp :type Primitive%20Component%20Object%20Reference) (OtherBodyIndex :type Integer))
  (Rendering|SetVisibility (Variables|Default|GetWidget) false false))

(event EventBeginPlay)

(event Collision|EventActorBeginOverlap
  (params (OtherActor :type Actor%20Object%20Reference)))

(event EventTick
  (params (DeltaSeconds :type Float%20%28single-precision%29))
  (bind _asbp_super_side_scroller_main_character (Utilities|Casting|CastToBP_SuperSideScroller_MainCharacter (Game|Player|GetPlayerPawn 0)))
  (if (Math|Boolean|ANDBoolean (Variables|/Game/MainCharacter/Blueprints/BP_SuperSideScroller_MainCharacter.BP_SuperSideScroller_MainCharacter_C|Getsign _asbp_super_side_scroller_main_character) (Variables|Default|Getplayer%20overlap) (not (Variables|/Game/MainCharacter/Blueprints/BP_SuperSideScroller_MainCharacter.BP_SuperSideScroller_MainCharacter_C|Getstage3cat1 _asbp_super_side_scroller_main_character)))
    (CallFunction|Npcchatlog)
    (bind _returnvalue (UserInterface|CreateWidget "/Game/objects/cats/WBP_catDialogue1.WBP_catDialogue1_C" (Game|GetPlayerController 0)))
    (UserInterface|Viewport|AddtoViewport _returnvalue 0)
    (elif (Variables|/Game/MainCharacter/Blueprints/BP_SuperSideScroller_MainCharacter.BP_SuperSideScroller_MainCharacter_C|Getstage3cat1 _asbp_super_side_scroller_main_character)
      (Components|Animation|SetAnimation (Variables|Default|GetSkeletalMesh) "/Game/asset/Cat_Simple/Cat/Animations/Anim_Cat_Simple_Caress_lie.Anim_Cat_Simple_Caress_lie"))))

(fn ConstructionScript)

(fn Npcchatlog
  (bind _asgi_stage (Utilities|Casting|CastToGI_stage (Game|GetGameInstance)))
  (Math|Integer|IncrementInt (Variables|/Game/MainCharacter/Blueprints/GI_stage.GI_stage_C|Getnpcchat _asgi_stage)
    (:%20%20
      (bind _returnvalue (Game|GetCurrentLevelName true))
      (if (Utilities|Enum|Equal(Enum) _returnvalue "Stage1_2")
        (Math|Integer|IncrementInt (Variables|/Game/MainCharacter/Blueprints/GI_stage.GI_stage_C|Getnpcchat1 _asgi_stage)
          (:%20%20
            _))
        (elif (or (Utilities|Enum|Equal(Enum) _returnvalue "Stage2_2A") (Utilities|Enum|Equal(Enum) _returnvalue "Stage2_2B"))
          (Math|Integer|IncrementInt (Variables|/Game/MainCharacter/Blueprints/GI_stage.GI_stage_C|Getnpcchat2 _asgi_stage)
            (:%20%20
              _))
          (elif (Utilities|Enum|Equal(Enum) _returnvalue "Stage3_2")
            (Math|Integer|IncrementInt (Variables|/Game/MainCharacter/Blueprints/GI_stage.GI_stage_C|Getnpcchat2 _asgi_stage)
              (:%20%20
                _)))))
      (return))))