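; BP_fishingpole is a one-time fishing pole pickup that destroys itself on BeginPlay if the game instance already records it as collected.
; When the player's main capsule overlaps its sphere, it sets the fishing pole flag on the character and GI_stage and increments two item counters.
; If save slot "1" exists, it also zeroes the target catnip count in the save and on the player.
; The actor then destroys itself.
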(event OnComponentBeginOverlap(Sphere)
  (params (OverlappedComponent :type Primitive%20Component%20Object%20Reference) (OtherActor :type Actor%20Object%20Reference) (OtherComp :type Primitive%20Component%20Object%20Reference) (OtherBodyIndex :type Integer) (bFromSweep :type Boolean) (SweepResult :type Hit%20Result%20Structure%20%28by%20ref%29))
  (bind _asbp_super_side_scroller_main_character (Utilities|Casting|CastToBP_SuperSideScroller_MainCharacter OtherActor))
  (if (== OtherComp (Variables|/Game/MainCharacter/Blueprints/BP_SuperSideScroller_MainCharacter.BP_SuperSideScroller_MainCharacter_C|GetmainCapsule _asbp_super_side_scroller_main_character))
    (Variables|/Game/MainCharacter/Blueprints/BP_SuperSideScroller_MainCharacter.BP_SuperSideScroller_MainCharacter_C|Setfishingpole _asbp_super_side_scroller_main_character true)
    (bind _asgi_stage (Utilities|Casting|CastToGI_stage (Game|GetGameInstance)))
    (Math|Integer|IncrementInt (Variables|/Game/MainCharacter/Blueprints/GI_stage.GI_stage_C|Getitem3 _asgi_stage)
      (:%20%20
        (Math|Integer|IncrementInt (Variables|/Game/MainCharacter/Blueprints/GI_stage.GI_stage_C|Getitem _asgi_stage)
          (:%20%20
            (Variables|/Game/MainCharacter/Blueprints/GI_stage.GI_stage_C|Setfishingpole _asgi_stage true)
            (bind _returnvalue (SaveGame|DoesSaveGameExist "1"))
            (if _returnvalue
              (bind _returnvalue_2 (SaveGame|LoadGamefromSlot "1"))
              (bind _asbp_saveobject (Utilities|Casting|CastToBP_saveobject _returnvalue_2))
              (bind _asbp_super_side_scroller_main_character_2 (Utilities|Casting|CastToBP_SuperSideScroller_MainCharacter (Game|GetPlayerCharacter 0)))
              (bind _output_get (Variables|/Game/objects/checkpoint/BP_saveobject.BP_saveobject_C|Setcounttargetcatnip _asbp_saveobject 0))
              (Variables|/Game/MainCharacter/Blueprints/BP_SuperSideScroller_MainCharacter.BP_SuperSideScroller_MainCharacter_C|Setinitcounttargetcatnip _asbp_super_side_scroller_main_character_2 _output_get)
              (SaveGame|SaveGametoSlot _asbp_saveobject "1"))
            (Actor|DestroyActor)))))))

(event EventBeginPlay
  (bind _asgi_stage (Utilities|Casting|CastToGI_stage (Game|GetGameInstance)))
  (if (Variables|/Game/MainCharacter/Blueprints/GI_stage.GI_stage_C|Getfishingpole _asgi_stage)
    (Actor|DestroyActor)))

(event Collision|EventActorBeginOverlap
  (params (OtherActor :type Actor%20Object%20Reference)))

(event EventTick
  (params (DeltaSeconds :type Float%20%28single-precision%29)))

(fn ConstructionScript)