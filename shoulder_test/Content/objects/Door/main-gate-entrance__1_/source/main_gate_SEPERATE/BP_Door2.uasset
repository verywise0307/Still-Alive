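; BP_Door2 is a double gate that opens when the side-scroller main character enters its box trigger and the GI_stage game instance has HasKey2 set.
; Two timelines animate the roll of the left and right door meshes, with a creak sound gated to play once.
; Without the key, it plays a locked sound and sets IsLocked on the character, gated by a DoOnce that resets when the overlap ends.
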(event OnComponentBeginOverlap(Box)
  (params (OverlappedComponent :type Primitive%20Component%20Object%20Reference) (OtherActor :type Actor%20Object%20Reference) (OtherComp :type Primitive%20Component%20Object%20Reference) (OtherBodyIndex :type Integer) (bFromSweep :type Boolean) (SweepResult :type Hit%20Result%20Structure%20%28by%20ref%29))
  (bind _asbp_super_side_scroller_main_character (Utilities|Casting|CastToBP_SuperSideScroller_MainCharacter OtherActor))
  (bind _asgi_stage (Utilities|Casting|CastToGI_stage (Game|GetGameInstance)))
  (if (Variables|/Game/MainCharacter/Blueprints/GI_stage.GI_stage_C|GetHasKey2 _asgi_stage)
    (Utilities|FlowControl|Sequence
      (:then_0
        (bind _doorratation (Timeline|DoorOpen Play)
          (:Update
            (Transformation|SetRelativeRotation (Variables|Default|GetDoor_Right) (Math|Rotator|MakeRotator _doorratation 87.0 9e+01) false false)
            (Utilities|FlowControl|DoOnce false
              (:Completed
                (Audio|PlaySoundatLocation "/Game/Sound/Scary_Door_Creak_Sound_Effect.Scary_Door_Creak_Sound_Effect" "0, 0, 0" "0, 0, 0" 1.0 1.0 0.0 0 0 0 0))))))
      (:then_1
        (bind _doorrotation (Timeline|타임라인 Play)
          (:Update
            (Transformation|SetRelativeRotation (Variables|Default|GetDoor_Left) (Math|Rotator|MakeRotator _doorrotation 93.0 9e+01) false false)))))
    (else
      (Utilities|FlowControl|DoOnce false
        (:Completed
          (Audio|PlaySoundatLocation "/Game/Sound/lockeddoor__online-audio-converter_com_.lockeddoor__online-audio-converter_com_" "0, 0, 0" "0, 0, 0" 1.0 1.0 0.0 0 0 0 0)
          (Variables|/Game/MainCharacter/Blueprints/BP_SuperSideScroller_MainCharacter.BP_SuperSideScroller_MainCharacter_C|SetIsLocked _asbp_super_side_scroller_main_character true))))))

(event OnComponentEndOverlap(Box)
  (params (OverlappedComponent :type Primitive%20Component%20Object%20Reference) (OtherActor :type Actor%20Object%20Reference) (OtherComp :type Primitive%20Component%20Object%20Reference) (OtherBodyIndex :type Integer))
  (Utilities|FlowControl|DoOnce false) ; enters at Reset
)

(fn ConstructionScript)