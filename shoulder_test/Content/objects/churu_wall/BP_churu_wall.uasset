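; A pushable wall object that the side-scroller character can topple once with physics.
; Overlap between the character's InteractiveBox and the Playeroverlap component toggles whether it can be pushed.
; Each Tick, while BoyGameMode reports pushing, it enables physics on Sphere and applies X-axis torque scaled by push direction.
; When Groundoverlap meets a groundcheck actor, physics stops and HasBeenFlipped blocks further pushing.
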(event OnComponentBeginOverlap(playeroverlap)
  (params (OverlappedComponent :type Primitive%20Component%20Object%20Reference) (OtherActor :type Actor%20Object%20Reference) (OtherComp :type Primitive%20Component%20Object%20Reference) (OtherBodyIndex :type Integer) (bFromSweep :type Boolean) (SweepResult :type Hit%20Result%20Structure%20%28by%20ref%29))
  (bind _asbp_super_side_scroller_main_character (Utilities|Casting|CastToBP_SuperSideScroller_MainCharacter OtherActor))
  (if (and (Class|PrimitiveComponent|IsOverlappingComponent (Variables|/Game/MainCharacter/Blueprints/BP_SuperSideScroller_MainCharacter.BP_SuperSideScroller_MainCharacter_C|GetinteractiveBox _asbp_super_side_scroller_main_character) (Variables|Default|Getplayeroverlap)) (not (Variables|Default|GethasBeenFlipped)))
    (Variables|Default|Setcanpush true)))

(event OnComponentEndOverlap(playeroverlap)
  (params (OverlappedComponent :type Primitive%20Component%20Object%20Reference) (OtherActor :type Actor%20Object%20Reference) (OtherComp :type Primitive%20Component%20Object%20Reference) (OtherBodyIndex :type Integer))
  (bind _asbp_super_side_scroller_main_character (Utilities|Casting|CastToBP_SuperSideScroller_MainCharacter OtherActor))
  (if (Class|PrimitiveComponent|IsOverlappingComponent (Variables|/Game/MainCharacter/Blueprints/BP_SuperSideScroller_MainCharacter.BP_SuperSideScroller_MainCharacter_C|GetinteractiveBox _asbp_super_side_scroller_main_character) (Variables|Default|Getplayeroverlap))
    (Variables|Default|Setcanpush false)))

(event OnComponentBeginOverlap(groundoverlap)
  (params (OverlappedComponent :type Primitive%20Component%20Object%20Reference) (OtherActor :type Actor%20Object%20Reference) (OtherComp :type Primitive%20Component%20Object%20Reference) (OtherBodyIndex :type Integer) (bFromSweep :type Boolean) (SweepResult :type Hit%20Result%20Structure%20%28by%20ref%29))
  (Utilities|Casting|CastTogroundcheck OtherActor)
  (Physics|SetSimulatePhysics (Variables|Default|GetSphere) false)
  (Variables|Default|SethasBeenFlipped true)
  (Development|PrintString "Hello"))

(event EventBeginPlay)

(event Collision|EventActorBeginOverlap
  (params (OtherActor :type Actor%20Object%20Reference)))

(event EventTick
  (params (DeltaSeconds :type Float%20%28single-precision%29))
  (bind _sphere (Variables|Default|GetSphere))
  (bind _asboy_game_mode (Utilities|Casting|CastToBoyGameMode (Game|GetGameMode)))
  (if (Math|Boolean|ANDBoolean (Variables|/Game/MainCharacter/Blueprints/BoyGameMode.BoyGameMode_C|GetIspushing _asboy_game_mode) (Variables|Default|Getcanpush) (not (Variables|Default|GethasBeenFlipped)))
    (Physics|SetSimulatePhysics _sphere true)
    (Class|PrimitiveComponent|AddTorqueinDegrees _sphere (Math|Vector|MakeVector (* (Variables|/Game/MainCharacter/Blueprints/BoyGameMode.BoyGameMode_C|Getpusingdirection _asboy_game_mode) -1e+03) 0.0 0.0) "None" true)))

(fn ConstructionScript)