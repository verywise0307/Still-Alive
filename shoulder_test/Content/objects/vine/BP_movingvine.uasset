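; BP_movingvine is a vine actor that moves using an InterpToMovement component.
; The construction script copies the Duration variable into the component to set its travel time.
; On BeginPlay the movement is switched off, then restarted at once if Delay is zero, or by a timer calling startmoving once Delay elapses.
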(event EventBeginPlay
  (bind _interptomovement (Variables|Default|GetInterpToMovement))
  (bind _delay (Variables|Default|Getdelay))
  (Components|Activation|SetActive (Variables|Default|GetInterpToMovement) false false)
  (if (== _delay 0.0)
    (Components|Activation|SetActive _interptomovement true false)
    (Class|InterptoMovementComponent|RestartMovement _interptomovement 1.0)
    (else
      (Utilities|Time|SetTimerbyFunctionName 0 "startmoving" _delay))))

(event Collision|EventActorBeginOverlap
  (params (OtherActor :type Actor%20Object%20Reference)))

(event EventTick
  (params (DeltaSeconds :type Float%20%28single-precision%29)))

(fn ConstructionScript
  (Variables|/Script/Engine.InterpToMovementComponent|SetDuration (Variables|Default|GetInterpToMovement) (Variables|Default|Getduration)))

(fn Startmoving
  (bind _interptomovement (Variables|Default|GetInterpToMovement))
  (Components|Activation|SetActive _interptomovement true false)
  (Class|InterptoMovementComponent|RestartMovement _interptomovement 1.0))