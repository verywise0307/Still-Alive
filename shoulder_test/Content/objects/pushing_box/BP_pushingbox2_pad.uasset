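; BP_pushingbox2_pad is a jump pad that bounces the side-scroller main character upward.
; When the character's Foot component enters Jumptrigger, LaunchCharacter applies a Z velocity that negates the capsule's current vertical physics velocity plus a fixed boost.
; It then calls Jumplog on the character and plays a jump sound at the world origin.
; BeginPlay, Tick and the construction script add no logic.
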(event OnComponentBeginOverlap(jumptrigger)
  (params (OverlappedComponent :type Primitive%20Component%20Object%20Reference) (OtherActor :type Actor%20Object%20Reference) (OtherComp :type Primitive%20Component%20Object%20Reference) (OtherBodyIndex :type Integer) (bFromSweep :type Boolean) (SweepResult :type Hit%20Result%20Structure%20%28by%20ref%29))
  (bind _asbp_super_side_scroller_main_character (Utilities|Casting|CastToBP_SuperSideScroller_MainCharacter OtherActor))
  (if (== OtherComp (Variables|/Game/MainCharacter/Blueprints/BP_SuperSideScroller_MainCharacter.BP_SuperSideScroller_MainCharacter_C|Getfoot _asbp_super_side_scroller_main_character))
    (bind _returnvalue (Physics|GetPhysicsLinearVelocity (Variables|/Script/Engine.Character|GetCapsuleComponent _asbp_super_side_scroller_main_character) "None"))
    (Character|LaunchCharacter _asbp_super_side_scroller_main_character (Math|Vector|MakeVector 0.0 0.0 (+ (* (.z _returnvalue) -1.0) 1.5e+03)) false false)
    (Default|Jumplog _asbp_super_side_scroller_main_character)
    (Audio|PlaySoundatLocation "/Game/Sound/jump__online-audio-converter_com_.jump__online-audio-converter_com_" "0, 0, 0" "0, 0, 0" 1.0 1.0 0.0 0 0 0 0)))

(event EventBeginPlay)

(event Collision|EventActorBeginOverlap
  (params (OtherActor :type Actor%20Object%20Reference)))

(event EventTick
  (params (DeltaSeconds :type Float%20%28single-precision%29))
  (|CallParentFunction DeltaSeconds) ; 지금 이 노드는 비활성 상태입니다. \n핀을 끌어서 다른 노드를 연결하면 활성화됩니다.
)

(fn ConstructionScript
  (|CallParentFunction))