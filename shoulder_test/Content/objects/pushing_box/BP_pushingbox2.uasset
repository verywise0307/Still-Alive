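; Pushable box for the side-scroller that the player slides along Y and that falls when it leaves the ground.
; Overlapping the character's InteractiveBox enables pushing; Tick then nudges the mesh by a fixed step following player velocity, gated by game mode Ispushing.
; Falling uses exponentially growing Velocity; ground overlaps and mesh hits land it on groundcheck actors or other boxes.
; Touching a groundcheck with Wallbox permanently halts movement.
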(event OnComponentEndOverlap(ground)
  (params (OverlappedComponent :type Primitive%20Component%20Object%20Reference) (OtherActor :type Actor%20Object%20Reference) (OtherComp :type Primitive%20Component%20Object%20Reference) (OtherBodyIndex :type Integer))
  ;[1 1 1] new
  (Utilities|Casting|CastTogroundcheck OtherActor)
  (Variables|Default|Setcanfall true))

(event OnComponentBeginOverlap(ground)
  (params (OverlappedComponent :type Primitive%20Component%20Object%20Reference) (OtherActor :type Actor%20Object%20Reference) (OtherComp :type Primitive%20Component%20Object%20Reference) (OtherBodyIndex :type Integer) (bFromSweep :type Boolean) (SweepResult :type Hit%20Result%20Structure%20%28by%20ref%29))
  ;[1 1 1] new
  (Utilities|Casting|CastTogroundcheck OtherActor
    (:then
      (if (Variables|Default|Getready)
        (Variables|Default|Setcanfall false :!label _label)))
    (:CastFailed
      (if (not (== self OtherActor))
        (bind _asbp_pushingbox_2 (Utilities|Casting|CastToBP_pushingbox2 OtherActor))
        (if (== (Variables|BP_pushingbox2_C|Gettopbox _asbp_pushingbox_2) OtherComp)
          (goto _label))))))

(event OnComponentBeginOverlap(playeroverlapbox)
  (params (OverlappedComponent :type Primitive%20Component%20Object%20Reference) (OtherActor :type Actor%20Object%20Reference) (OtherComp :type Primitive%20Component%20Object%20Reference) (OtherBodyIndex :type Integer) (bFromSweep :type Boolean) (SweepResult :type Hit%20Result%20Structure%20%28by%20ref%29))
  ;[1 1 1] new
  (bind _asbp_super_side_scroller_main_character (Utilities|Casting|CastToBP_SuperSideScroller_MainCharacter OtherActor))
  (if (== OtherComp (Variables|/Game/MainCharacter/Blueprints/BP_SuperSideScroller_MainCharacter.BP_SuperSideScroller_MainCharacter_C|GetinteractiveBox _asbp_super_side_scroller_main_character))
    (Variables|/Script/shoulder_test.shoulder_testCharacter|Setcanpush _asbp_super_side_scroller_main_character true)
    (Variables|Default|Setplayeroverlap true)))

(event OnComponentEndOverlap(playeroverlapbox)
  (params (OverlappedComponent :type Primitive%20Component%20Object%20Reference) (OtherActor :type Actor%20Object%20Reference) (OtherComp :type Primitive%20Component%20Object%20Reference) (OtherBodyIndex :type Integer))
  ;[1 1 1] new
  (bind _asbp_super_side_scroller_main_character (Utilities|Casting|CastToBP_SuperSideScroller_MainCharacter OtherActor))
  (if (== OtherComp (Variables|/Game/MainCharacter/Blueprints/BP_SuperSideScroller_MainCharacter.BP_SuperSideScroller_MainCharacter_C|GetinteractiveBox _asbp_super_side_scroller_main_character))
    (Variables|/Script/shoulder_test.shoulder_testCharacter|Setcanpush _asbp_super_side_scroller_main_character false)
    (Variables|Default|Setplayeroverlap false)))

(event OnComponentHit(StaticMesh)
  (params (HitComponent :type Primitive%20Component%20Object%20Reference) (OtherActor :type Actor%20Object%20Reference) (OtherComp :type Primitive%20Component%20Object%20Reference) (NormalImpulse :type Vector :default "0, 0, 0") (Hit :type Hit%20Result%20Structure%20%28by%20ref%29))
  ;[1 1 1] new
  (if (and (Variables|Default|Getcanfall) (Variables|Default|Getready))
    (Utilities|Casting|CastTogroundcheck OtherActor
      (:then
        (Variables|Default|Setcanfall false :!label _label)
        (Variables|Default|Setready false))
      (:CastFailed
        (if (not (== OtherActor self))
          (Utilities|Casting|CastToBP_pushingbox2 OtherActor)
          (goto _label))))))

(event OnComponentBeginOverlap(groundBox2)
  (params (OverlappedComponent :type Primitive%20Component%20Object%20Reference) (OtherActor :type Actor%20Object%20Reference) (OtherComp :type Primitive%20Component%20Object%20Reference) (OtherBodyIndex :type Integer) (bFromSweep :type Boolean) (SweepResult :type Hit%20Result%20Structure%20%28by%20ref%29))
  ;[1 1 1] new
  (Utilities|Casting|CastTogroundcheck OtherActor
    (:then
      (Variables|Default|Setready true :!label _label))
    (:CastFailed
      (if (not (== self OtherActor))
        (bind _asbp_pushingbox_2 (Utilities|Casting|CastToBP_pushingbox2 OtherActor))
        (if (== (Variables|BP_pushingbox2_C|Gettopbox _asbp_pushingbox_2) OtherComp)
          (goto _label))))))

(event OnComponentBeginOverlap(wallbox)
  (params (OverlappedComponent :type Primitive%20Component%20Object%20Reference) (OtherActor :type Actor%20Object%20Reference) (OtherComp :type Primitive%20Component%20Object%20Reference) (OtherBodyIndex :type Integer) (bFromSweep :type Boolean) (SweepResult :type Hit%20Result%20Structure%20%28by%20ref%29))
  ;[1 1 1] new
  (Utilities|Casting|CastTogroundcheck OtherActor)
  (Variables|Default|SethitWall true))

(event OnComponentEndOverlap(groundBox2)
  (params (OverlappedComponent :type Primitive%20Component%20Object%20Reference) (OtherActor :type Actor%20Object%20Reference) (OtherComp :type Primitive%20Component%20Object%20Reference) (OtherBodyIndex :type Integer))
  ;[1 1 1] new
  (Utilities|Casting|CastTogroundcheck OtherActor)
  (Variables|Default|Setready false))

(event EventTick
  (params (DeltaSeconds :type Float%20%28single-precision%29))
  (bind _staticmesh (Variables|Default|GetStaticMesh))
  (bind _canfall (Variables|Default|Getcanfall))
  ;[1 1 1] new
  (bind _asboy_game_mode (Utilities|Casting|CastToBoyGameMode (Game|GetGameMode)))
  (if (and (or (and (Variables|/Game/MainCharacter/Blueprints/BoyGameMode.BoyGameMode_C|GetIspushing _asboy_game_mode) (Variables|Default|Getplayeroverlap)) _canfall) (not (Variables|Default|GethitWall)))
    (if _canfall
      (bind _output_get (Variables|Default|Setvelocity (* (Variables|Default|Getvelocity) (Math|Float|Power 1.5 DeltaSeconds))))
      (Transformation|AddWorldOffset _staticmesh (Math|Vector|MakeVector 0.0 0.0 _output_get) false false)
      (else
        (Transformation|AddWorldOffset _staticmesh (Math|Vector|MakeVector 0.0 (Math|Float|SelectFloat 1.5 -1.5 (> (.y (Transformation|GetVelocity (Game|Player|GetPlayerPawn 0))) 0.0)) 0.0) false false)))))

(fn ConstructionScript
  (Components|StaticMesh|SetStaticMesh (Variables|Default|GetStaticMesh) (Variables|Default|Getbox%20StaticMesh)))