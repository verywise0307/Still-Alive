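; Catnip area actor for the stage 3 weapon pickup mechanic, which rains falling catnip and converts collected catnip into weapons.
; A looping one-second timer spawns BP_fallingcatnip at a random XY within the Range-based area, raised above the actor.
; The construction script scales the Box by Range.
; Tick polls the player character, resetting CatnipCount and incrementing WeaponCount once the count reaches ten.
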(event EventBeginPlay
  (Utilities|Time|SetTimerbyFunctionName 0 "spawn catnip" 1.0 true))

(event Collision|EventActorBeginOverlap
  (params (OtherActor :type Actor%20Object%20Reference)))

(event EventTick
  (params (DeltaSeconds :type Float%20%28single-precision%29))
  (bind _asbp_super_side_scroller_main_character (Utilities|Casting|CastToBP_SuperSideScroller_MainCharacter (Game|GetPlayerCharacter 0)))
  (if (>= (Variables|/Script/shoulder_test.shoulder_testCharacter|Getcatnip_count _asbp_super_side_scroller_main_character) 10)
    (Variables|/Script/shoulder_test.shoulder_testCharacter|Setcatnip_count _asbp_super_side_scroller_main_character 0)
    (bind _result (Math|Integer|IncrementInt (Variables|/Script/shoulder_test.shoulder_testCharacter|Getweapon_count _asbp_super_side_scroller_main_character))
      (:%20%20
        (Variables|/Script/shoulder_test.shoulder_testCharacter|Setweapon_count _asbp_super_side_scroller_main_character _result)))))

(fn ConstructionScript
  (bind _range (Variables|Default|Getrange))
  (Transformation|SetRelativeScale3D (Variables|Default|GetBox) (Math|Vector|MakeVector _range _range _range)))

(fn SpawnCatnip
  (bind _returnvalue (Transformation|GetActorLocation))
  (bind _range (Variables|Default|Getrange))
  (bind _returnvalue_2 (* _range 32.0))
  (bind _returnvalue_3 (* _returnvalue_2 -1.0))
  (Math|Random|SetRandomStreamSeed (Math|Random|MakeRandomStream (Math|Float|Truncate (Utilities|Time|GetGameTimeinSeconds))) 5)
  (bind _returnvalue_4 (Game|SpawnActorfromClass "/Game/objects/weapon/stage3/BP_fallingcatnip.BP_fallingcatnip_C" (Math|Transform|MakeTransform (Math|Vector|MakeVector (+ (Math|Random|RandomFloatinRange _returnvalue_3 _returnvalue_2) (.x _returnvalue)) (+ (Math|Random|RandomFloatinRange _returnvalue_3 _returnvalue_2) (.y _returnvalue)) (+ _returnvalue_2 (.z _returnvalue))) "0, 0, 0" "1.000000,1.000000,1.000000") "Undefined" 0 0))
  (Transformation|AttachActorToActor _returnvalue_4 0 "None" "KeepRelative" "KeepRelative" "KeepRelative" true))