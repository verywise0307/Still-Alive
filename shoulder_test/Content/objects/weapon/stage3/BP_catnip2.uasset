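; Catnip pickup in the stage 3 weapon folder that the side-scroller main character collects by hitting its mesh.
; A hit adds two to CatnipCount, increments WeaponCount whenever the total is at least ten, then destroys the actor.
; A sphere overlap by any actor shows a widget only the first time, hiding it after a short delay or when an overlap ends.
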(event OnComponentHit(StaticMesh)
  (params (HitComponent :type Primitive%20Component%20Object%20Reference) (OtherActor :type Actor%20Object%20Reference) (OtherComp :type Primitive%20Component%20Object%20Reference) (NormalImpulse :type Vector :default "0, 0, 0") (Hit :type Hit%20Result%20Structure%20%28by%20ref%29))
  (bind _asbp_super_side_scroller_main_character (Utilities|Casting|CastToBP_SuperSideScroller_MainCharacter OtherActor))
  (bind _output_get (Variables|/Script/shoulder_test.shoulder_testCharacter|Setcatnip_count _asbp_super_side_scroller_main_character (+ (Variables|/Script/shoulder_test.shoulder_testCharacter|Getcatnip_count _asbp_super_side_scroller_main_character) 2)))
  (if (>= _output_get 10)
    (Variables|/Script/shoulder_test.shoulder_testCharacter|Setweapon_count _asbp_super_side_scroller_main_character (+ (Variables|/Script/shoulder_test.shoulder_testCharacter|Getweapon_count _asbp_super_side_scroller_main_character) 1)))
  (Actor|DestroyActor))

(event OnComponentBeginOverlap(Sphere)
  (params (OverlappedComponent :type Primitive%20Component%20Object%20Reference) (OtherActor :type Actor%20Object%20Reference) (OtherComp :type Primitive%20Component%20Object%20Reference) (OtherBodyIndex :type Integer) (bFromSweep :type Boolean) (SweepResult :type Hit%20Result%20Structure%20%28by%20ref%29))
  (bind _widget (Variables|Default|GetWidget))
  (Utilities|FlowControl|DoOnce false
    (:Completed
      (Rendering|SetVisibility _widget true false)
      (Utilities|FlowControl|Delay 3.0)
      (Rendering|SetVisibility _widget false false))))

(event OnComponentEndOverlap(Sphere)
  (params (OverlappedComponent :type Primitive%20Component%20Object%20Reference) (OtherActor :type Actor%20Object%20Reference) (OtherComp :type Primitive%20Component%20Object%20Reference) (OtherBodyIndex :type Integer))
  (Rendering|SetVisibility (Variables|Default|GetWidget) false false))

(event EventBeginPlay)

(event Collision|EventActorBeginOverlap
  (params (OtherActor :type Actor%20Object%20Reference)))

(event EventTick
  (params (DeltaSeconds :type Float%20%28single-precision%29)))

(fn ConstructionScript)