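; BP_throwingcan is a stage 1 thrown-can weapon that damages BP_Enemy2 on contact.
; When its Box overlaps that enemy's HitCapsule, it subtracts a fixed amount of HP and destroys itself once the stats are recorded.
; It increments the throwing-attack hit count in GI_stage and, if still unset, records the first-attack time as seconds since midnight.
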(event OnComponentBeginOverlap(Box)
  (params (OverlappedComponent :type Primitive%20Component%20Object%20Reference) (OtherActor :type Actor%20Object%20Reference) (OtherComp :type Primitive%20Component%20Object%20Reference) (OtherBodyIndex :type Integer) (bFromSweep :type Boolean) (SweepResult :type Hit%20Result%20Structure%20%28by%20ref%29))
  (bind _returnvalue (Math|DateTime|Now))
  (bind _asbp_enemy_2 (Utilities|Casting|CastToBP_Enemy2 OtherActor))
  (if (== (Variables|/Game/enemy/Blueprints/BP_Enemy2.BP_Enemy2_C|GethitCapsule _asbp_enemy_2) OtherComp)
    (Variables|/Game/enemy/Blueprints/BP_Enemy2.BP_Enemy2_C|SetHP _asbp_enemy_2 (- (Variables|/Game/enemy/Blueprints/BP_Enemy2.BP_Enemy2_C|GetHP _asbp_enemy_2) 10))
    (bind _asgi_stage (Utilities|Casting|CastToGI_stage (Game|GetGameInstance)))
    (Math|Integer|IncrementInt (Variables|/Game/MainCharacter/Blueprints/GI_stage.GI_stage_C|Getstage1throwingattackhitcount _asgi_stage)
      (:%20%20
        (if (== (Variables|/Game/MainCharacter/Blueprints/GI_stage.GI_stage_C|Getstage1firstattack _asgi_stage) 0.0)
          (Variables|/Game/MainCharacter/Blueprints/GI_stage.GI_stage_C|Setstage1firstattack _asgi_stage (Math|Conversions|ToFloat(Integer) (+ (* (.hour _returnvalue) 3600) (* (.minute _returnvalue) 60) (.second _returnvalue)))))
        (Actor|DestroyActor)))))

(event EventBeginPlay)

(event Collision|EventActorBeginOverlap
  (params (OtherActor :type Actor%20Object%20Reference)))

(event EventTick
  (params (DeltaSeconds :type Float%20%28single-precision%29)))

(fn ConstructionScript)