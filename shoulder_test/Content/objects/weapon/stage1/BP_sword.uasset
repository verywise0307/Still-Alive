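; BP_sword is a sword pickup for the side-scroller that floats up and down until collected.
; On overlap with the main character, it sets that character's Weapon to 1 and destroys itself.
; Tick accumulates running time and adds a scaled sine of it to the static mesh's current world Z, so the bobbing is frame-rate dependent.
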(event EventBeginPlay)

(event Collision|EventActorBeginOverlap
  (params (OtherActor :type Actor%20Object%20Reference))
  (bind _asbp_super_side_scroller_main_character (Utilities|Casting|CastToBP_SuperSideScroller_MainCharacter OtherActor))
  (Variables|/Script/shoulder_test.shoulder_testCharacter|Setweapon _asbp_super_side_scroller_main_character 1)
  (Actor|DestroyActor))

(event EventTick
  (params (DeltaSeconds :type Float%20%28single-precision%29))
  (bind _staticmesh (Variables|Default|GetStaticMesh))
  (bind _returnvalue (Transformation|GetWorldLocation _staticmesh))
  (bind (_x _y _z) (Math|Vector|BreakVector _returnvalue))
  (bind _output_get (Variables|Default|SetRunningTime (+ DeltaSeconds (Variables|Default|GetRunningTime))))
  (bind _output_get_2 (Variables|Default|SetNewLocation (Math|Vector|MakeVector _x _y (+ (/ (Math|Trig|Sin(Radians) _output_get) 4.0) _z))))
  (Transformation|SetWorldLocation (Variables|Default|GetStaticMesh) _output_get_2 false false))

(fn ConstructionScript)