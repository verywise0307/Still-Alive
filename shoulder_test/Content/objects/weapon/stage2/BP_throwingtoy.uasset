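; Thrown toy projectile for stage 2 that lands on the ground and breaks against certain other objects.
; Overlapping a groundcheck stops its movement and registers it in GI_stage as the current toy, then clears that reference and destroys it after a delay.
; BreakingSphere uses a cast chain to destroy it on other throwing toys, falling toys, thrown yarn or boss barriers, ignoring the player, toy areas and boss post-process actors.
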(event OnComponentBeginOverlap(breakingSphere)
  (params (OverlappedComponent :type Primitive%20Component%20Object%20Reference) (OtherActor :type Actor%20Object%20Reference) (OtherComp :type Primitive%20Component%20Object%20Reference) (OtherBodyIndex :type Integer) (bFromSweep :type Boolean) (SweepResult :type Hit%20Result%20Structure%20%28by%20ref%29))
  (Utilities|Casting|CastToBP_SuperSideScroller_MainCharacter OtherActor
    (:CastFailed
      (Utilities|Casting|CastToBP_toyarea OtherActor
        (:CastFailed
          (Utilities|Casting|CastToBP_postprocessboss3 OtherActor
            (:CastFailed
              (bind _asbp_throwingtoy (Utilities|Casting|CastToBP_throwingtoy OtherActor)
                (:then
                  (if (== _asbp_throwingtoy self)
                    (Development|PrintString "hi")
                    (else
                      (Development|PrintString "Hello")
                      (Actor|DestroyActor :!label _label))))
                (:CastFailed
                  (Utilities|Casting|CastToBP_fallingtoy OtherActor
                    (:then
                      (goto _label))
                    (:CastFailed
                      (Utilities|Casting|CastToBP_throwingyarn OtherActor
                        (:then
                          (Actor|DestroyActor))
                        (:CastFailed
                          (Utilities|Casting|CastToBP_bossbarrier OtherActor)
                          (Actor|DestroyActor))))))))))))))

(event OnComponentHit(StaticMesh)
  (params (HitComponent :type Primitive%20Component%20Object%20Reference) (OtherActor :type Actor%20Object%20Reference) (OtherComp :type Primitive%20Component%20Object%20Reference) (NormalImpulse :type Vector :default "0, 0, 0") (Hit :type Hit%20Result%20Structure%20%28by%20ref%29)))

(event EventBeginPlay)

(event Collision|EventActorBeginOverlap
  (params (OtherActor :type Actor%20Object%20Reference))
  (Utilities|Casting|CastTogroundcheck OtherActor)
  (Game|Components|ProjectileMovement|StopSimulating (Variables|Default|GetProjectileMovement) (stale OnComponentHit(StaticMesh) Hit))
  (bind _asgi_stage (Utilities|Casting|CastToGI_stage (Game|GetGameInstance)))
  (Variables|/Game/MainCharacter/Blueprints/GI_stage.GI_stage_C|Settoy _asgi_stage true)
  (Variables|/Game/MainCharacter/Blueprints/GI_stage.GI_stage_C|SetBP_toy _asgi_stage self)
  (Utilities|FlowControl|Delay 5.0)
  (Variables|/Game/MainCharacter/Blueprints/GI_stage.GI_stage_C|SetBP_toy _asgi_stage 0)
  (Actor|DestroyActor))

(event EventTick
  (params (DeltaSeconds :type Float%20%28single-precision%29)))

(fn ConstructionScript)