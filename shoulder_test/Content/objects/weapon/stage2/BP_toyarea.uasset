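; BP_toyarea is a stage 2 area that rains falling toys from above.
; The construction script scales its Box uniformly by Range.
; From BeginPlay, a looping one-second timer runs spawn toy, which spawns one BP_fallingtoy for each BP_stage2enemy whose Throw flag is false.
; Toys appear at random X/Y within the Range-sized area, at its top height; the seeded random stream does not feed those random rolls.
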(event EventBeginPlay
  (Utilities|Time|SetTimerbyFunctionName 0 "spawn toy" 1.0 true))

(event Collision|EventActorBeginOverlap
  (params (OtherActor :type Actor%20Object%20Reference)))

(event EventTick
  (params (DeltaSeconds :type Float%20%28single-precision%29)))

(fn ConstructionScript
  (bind _range (Variables|Default|Getrange))
  (Transformation|SetRelativeScale3D (Variables|Default|GetBox) (Math|Vector|MakeVector _range _range _range)))

(fn SpawnToy
  (bind _returnvalue (Transformation|GetActorLocation))
  (bind _range (Variables|Default|Getrange))
  (bind _returnvalue_2 (* _range 32.0))
  (bind _returnvalue_3 (* _returnvalue_2 -1.0))
  (bind _outactors (Actor|GetAllActorsOfClass "/Game/enemy/stage2/BP_stage2enemy.BP_stage2enemy_C"))
  (for _array_element _outactors
    (if (not (Variables|/Game/enemy/stage2/BP_stage2enemy.BP_stage2enemy_C|Getthrow _array_element))
      (Math|Random|SetRandomStreamSeed (Math|Random|MakeRandomStream (Math|Float|Truncate (Utilities|Time|GetGameTimeinSeconds))) 5)
      (bind _returnvalue_4 (Game|SpawnActorfromClass "/Game/objects/weapon/stage2/BP_fallingtoy.BP_fallingtoy_C" (Math|Transform|MakeTransform (Math|Vector|MakeVector (+ (Math|Random|RandomFloatinRange _returnvalue_3 _returnvalue_2) (.x _returnvalue)) (+ (Math|Random|RandomFloatinRange _returnvalue_3 _returnvalue_2) (.y _returnvalue)) (+ _returnvalue_2 (.z _returnvalue))) "0, 0, 0" "1.000000,1.000000,1.000000") "Undefined" 0 0))
      (Transformation|AttachActorToActor _returnvalue_4 0 "None" "KeepRelative" "KeepRelative" "KeepRelative" true))))