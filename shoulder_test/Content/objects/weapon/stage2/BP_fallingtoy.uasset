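; BP_fallingtoy is a stage 2 falling toy that hurts the player until it lands, then becomes a weapon pickup.
; Its static mesh hit event drives everything: touching a groundcheck actor sets the Stay flag and starts a timed self-destruct.
; A player hit subtracts HP before landing, or increments WeaponCount and destroys the toy afterward.
; Hitting any other actor destroys it immediately.
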(event OnComponentHit(StaticMesh)
  (params (HitComponent :type Primitive%20Component%20Object%20Reference) (OtherActor :type Actor%20Object%20Reference) (OtherComp :type Primitive%20Component%20Object%20Reference) (NormalImpulse :type Vector :default "0, 0, 0") (Hit :type Hit%20Result%20Structure%20%28by%20ref%29))
  (bind _asbp_super_side_scroller_main_character (Utilities|Casting|CastToBP_SuperSideScroller_MainCharacter OtherActor)
    (:then
      (if (Variables|Default|Getstay)
        (bind _result (Math|Integer|IncrementInt (Variables|/Script/shoulder_test.shoulder_testCharacter|Getweapon_count _asbp_super_side_scroller_main_character))
          (:%20%20
            (Variables|/Script/shoulder_test.shoulder_testCharacter|Setweapon_count _asbp_super_side_scroller_main_character _result)
            (Actor|DestroyActor)))
        (else
          (Variables|/Game/MainCharacter/Blueprints/BP_SuperSideScroller_MainCharacter.BP_SuperSideScroller_MainCharacter_C|SetHP _asbp_super_side_scroller_main_character (- (Variables|/Game/MainCharacter/Blueprints/BP_SuperSideScroller_MainCharacter.BP_SuperSideScroller_MainCharacter_C|GetHP _asbp_super_side_scroller_main_character) 10)))))
    (:CastFailed
      (Utilities|Casting|CastTogroundcheck OtherActor
        (:then
          (Variables|Default|Setstay true)
          (Utilities|FlowControl|Delay 1e+01)
          (Actor|DestroyActor))
        (:CastFailed
          (Actor|DestroyActor))))))

(event EventBeginPlay)

(event Collision|EventActorBeginOverlap
  (params (OtherActor :type Actor%20Object%20Reference)))

(event EventTick
  (params (DeltaSeconds :type Float%20%28single-precision%29)))

(fn ConstructionScript)