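; BP_Ball is a side-scroller ball that reacts to the player pushing it, gradually shrinking as it is pushed.
; Box overlaps set a flag that gates per-tick logic, which treats non-zero player Y velocity as pushing.
; While pushing, it slows the player's walk speed, sets IsPushingBall on BoyGameMode and scales itself down slightly each frame.
; Stopping or leaving the box restores speed and clears the game mode flag.
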(event OnComponentBeginOverlap(Box)
  (params (OverlappedComponent :type Primitive%20Component%20Object%20Reference) (OtherActor :type Actor%20Object%20Reference) (OtherComp :type Primitive%20Component%20Object%20Reference) (OtherBodyIndex :type Integer) (bFromSweep :type Boolean) (SweepResult :type Hit%20Result%20Structure%20%28by%20ref%29))
  (if (== OtherActor (Variables|Default|GetPlayer%20ref))
    (Variables|Default|SetTick true)
    (else
      (Variables|Default|SetTick false))))

(event OnComponentEndOverlap(Box)
  (params (OverlappedComponent :type Primitive%20Component%20Object%20Reference) (OtherActor :type Actor%20Object%20Reference) (OtherComp :type Primitive%20Component%20Object%20Reference) (OtherBodyIndex :type Integer))
  (if (== OtherActor (Variables|Default|GetPlayer%20ref))
    (Variables|Default|SetTick false)
    (Variables|/Script/Engine.CharacterMovementComponent|SetMaxWalkSpeed (Variables|/Script/Engine.Character|GetCharacterMovement (Variables|Default|GetPlayer%20ref)) 5e+02)
    (bind _asboy_game_mode (Utilities|Casting|CastToBoyGameMode (Game|GetGameMode)))
    (Variables|/Game/MainCharacter/Blueprints/BoyGameMode.BoyGameMode_C|SetIsPushingBall _asboy_game_mode false)))

(event EventBeginPlay
  (bind _asbp_super_side_scroller_main_character (Utilities|Casting|CastToBP_SuperSideScroller_MainCharacter (Game|GetPlayerCharacter 0)))
  (Variables|Default|SetPlayer%20ref _asbp_super_side_scroller_main_character))

(event EventTick
  (params (DeltaSeconds :type Float%20%28single-precision%29))
  (bind _returnvalue (Transformation|GetActorScale3D))
  (bind _player_ref (Variables|Default|GetPlayer%20ref))
  (bind _charactermovement (Variables|/Script/Engine.Character|GetCharacterMovement _player_ref))
  (if (Variables|Default|GetTick)
    (if (!= (.Y (Math|Vector|BreakVector (Variables|/Script/Engine.MovementComponent|GetVelocity (Variables|/Script/Engine.Character|GetCharacterMovement (Variables|Default|GetPlayer%20ref))))) 0.0)
      (bind _asboy_game_mode (Utilities|Casting|CastToBoyGameMode (Game|GetGameMode)))
      (Variables|/Game/MainCharacter/Blueprints/BoyGameMode.BoyGameMode_C|SetIsPushingBall _asboy_game_mode true)
      (Variables|/Script/Engine.CharacterMovementComponent|SetMaxWalkSpeed _charactermovement 3e+02)
      (Transformation|SetActorScale3D (Math|Vector|MakeVector (* (.x _returnvalue) 0.999) (* (.y _returnvalue) 0.999) (* (.z _returnvalue) 0.999)))
      (Development|PrintString "444")
      (else
        (bind _asboy_game_mode_2 (Utilities|Casting|CastToBoyGameMode (Game|GetGameMode)))
        (Variables|/Game/MainCharacter/Blueprints/BoyGameMode.BoyGameMode_C|SetIsPushingBall _asboy_game_mode_2 false)
        (Variables|/Script/Engine.CharacterMovementComponent|SetMaxWalkSpeed _charactermovement 5e+02)))))

(fn ConstructionScript)