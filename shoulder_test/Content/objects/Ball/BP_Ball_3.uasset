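; Pushable ball for a side-scroller that gradually shrinks while the player pushes it.
; Sphere1 overlapping the player's InteractiveBox enables the Tick check for movement toward the ball with the push key held.
; Pushing flags BoyGameMode, slows walking and scales the actor down while preserving the Cable's world scale; otherwise walk speed is restored and BlockSphere velocity zeroed.
; MainSphere records groundcheck overlaps in Checkground, unread here.
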(event OnComponentBeginOverlap(Sphere)
  (params (OverlappedComponent :type Primitive%20Component%20Object%20Reference) (OtherActor :type Actor%20Object%20Reference) (OtherComp :type Primitive%20Component%20Object%20Reference) (OtherBodyIndex :type Integer) (bFromSweep :type Boolean) (SweepResult :type Hit%20Result%20Structure%20%28by%20ref%29)))

(event OnComponentEndOverlap(Sphere)
  (params (OverlappedComponent :type Primitive%20Component%20Object%20Reference) (OtherActor :type Actor%20Object%20Reference) (OtherComp :type Primitive%20Component%20Object%20Reference) (OtherBodyIndex :type Integer)))

(event OnComponentBeginOverlap(Sphere1)
  (params (OverlappedComponent :type Primitive%20Component%20Object%20Reference) (OtherActor :type Actor%20Object%20Reference) (OtherComp :type Primitive%20Component%20Object%20Reference) (OtherBodyIndex :type Integer) (bFromSweep :type Boolean) (SweepResult :type Hit%20Result%20Structure%20%28by%20ref%29))
  (bind _asbp_super_side_scroller_main_character (Utilities|Casting|CastToBP_SuperSideScroller_MainCharacter OtherActor))
  (if (== OtherComp (Variables|/Game/MainCharacter/Blueprints/BP_SuperSideScroller_MainCharacter.BP_SuperSideScroller_MainCharacter_C|GetinteractiveBox _asbp_super_side_scroller_main_character))
    (Variables|Default|SetTick true)))

(event OnComponentEndOverlap(Sphere1)
  (params (OverlappedComponent :type Primitive%20Component%20Object%20Reference) (OtherActor :type Actor%20Object%20Reference) (OtherComp :type Primitive%20Component%20Object%20Reference) (OtherBodyIndex :type Integer))
  (bind _asbp_super_side_scroller_main_character (Utilities|Casting|CastToBP_SuperSideScroller_MainCharacter OtherActor))
  (if (== OtherComp (Variables|/Game/MainCharacter/Blueprints/BP_SuperSideScroller_MainCharacter.BP_SuperSideScroller_MainCharacter_C|GetinteractiveBox _asbp_super_side_scroller_main_character))
    (Variables|Default|SetTick false)
    (Variables|/Script/Engine.CharacterMovementComponent|SetMaxWalkSpeed (Variables|/Script/Engine.Character|GetCharacterMovement (Variables|Default|GetPlayer%20ref)) 5e+02)
    (bind _asboy_game_mode (Utilities|Casting|CastToBoyGameMode (Game|GetGameMode)))
    (Variables|/Game/MainCharacter/Blueprints/BoyGameMode.BoyGameMode_C|SetIsPushingBall _asboy_game_mode false)))

(event OnComponentBeginOverlap(mainSphere)
  (params (OverlappedComponent :type Primitive%20Component%20Object%20Reference) (OtherActor :type Actor%20Object%20Reference) (OtherComp :type Primitive%20Component%20Object%20Reference) (OtherBodyIndex :type Integer) (bFromSweep :type Boolean) (SweepResult :type Hit%20Result%20Structure%20%28by%20ref%29))
  (Utilities|Casting|CastTogroundcheck OtherActor)
  (Variables|Default|Setcheckground true))

(event OnComponentEndOverlap(mainSphere)
  (params (OverlappedComponent :type Primitive%20Component%20Object%20Reference) (OtherActor :type Actor%20Object%20Reference) (OtherComp :type Primitive%20Component%20Object%20Reference) (OtherBodyIndex :type Integer))
  (Utilities|Casting|CastTogroundcheck OtherActor)
  (Variables|Default|Setcheckground false))

(event EventBeginPlay
  (bind _asbp_super_side_scroller_main_character (Utilities|Casting|CastToBP_SuperSideScroller_MainCharacter (Game|GetPlayerCharacter 0)))
  (Variables|Default|SetPlayer%20ref _asbp_super_side_scroller_main_character))

(event EventTick
  (params (DeltaSeconds :type Float%20%28single-precision%29))
  (bind _returnvalue (Transformation|GetActorLocation))
  (bind _returnvalue_2 (Transformation|GetActorScale3D))
  (bind _cable (Variables|Default|GetCable))
  (bind _player_ref (Variables|Default|GetPlayer%20ref))
  (bind _player_ref_2 (Variables|Default|GetPlayer%20ref))
  (bind _maincapsule (Variables|/Game/MainCharacter/Blueprints/BP_SuperSideScroller_MainCharacter.BP_SuperSideScroller_MainCharacter_C|GetmainCapsule _player_ref_2))
  (bind _charactermovement (Variables|/Script/Engine.Character|GetCharacterMovement _player_ref))
  (bind _returnvalue_3 (Math|Vector|GetForwardVector _maincapsule))
  (bind _returnvalue_4 (Transformation|GetWorldLocation _maincapsule))
  (if (Variables|Default|GetTick)
    (if (!= (.Y (Math|Vector|BreakVector (Variables|/Script/Engine.MovementComponent|GetVelocity (Variables|/Script/Engine.Character|GetCharacterMovement _player_ref_2)))) 0.0)
      (if (and (or (and (> (- (.y _returnvalue) (.y _returnvalue_4)) 0.0) (> (.y _returnvalue_3) 0.0)) (and (< (.y _returnvalue_3) 0.0) (> (- (.y _returnvalue_4) (.y _returnvalue)) 0.0))) (== (Variables|/Game/MainCharacter/Blueprints/BP_SuperSideScroller_MainCharacter.BP_SuperSideScroller_MainCharacter_C|GetFpushkey (Variables|Default|GetPlayer%20ref)) 1.0))
        (bind _asboy_game_mode (Utilities|Casting|CastToBoyGameMode (Game|GetGameMode)))
        (Variables|/Game/MainCharacter/Blueprints/BoyGameMode.BoyGameMode_C|SetIsPushingBall _asboy_game_mode true)
        (Variables|/Script/Engine.CharacterMovementComponent|SetMaxWalkSpeed _charactermovement 1e+02)
        (Variables|Default|Setcablescale (Transformation|GetWorldScale _cable))
        (Transformation|SetActorScale3D (Math|Vector|MakeVector (* (.x _returnvalue_2) 0.999) (* (.y _returnvalue_2) 0.999) (* (.z _returnvalue_2) 0.999)))
        (Transformation|SetWorldScale3D _cable (Variables|Default|Getcablescale))
        (else
          (bind _asboy_game_mode_2 (Utilities|Casting|CastToBoyGameMode (Game|GetGameMode) :!label _label))
          (Variables|/Game/MainCharacter/Blueprints/BoyGameMode.BoyGameMode_C|SetIsPushingBall _asboy_game_mode_2 false)
          (Variables|/Script/Engine.CharacterMovementComponent|SetMaxWalkSpeed _charactermovement 5e+02)
          (if true
            (Physics|SetPhysicsLinearVelocity (Variables|Default|GetblockSphere) "0, 0, 0" false "None"))))
      (else
        (goto _label)))))

(fn ConstructionScript)