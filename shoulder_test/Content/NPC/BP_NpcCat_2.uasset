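; Cat NPC for a side-scroller that shows dialogue when the player's main capsule touches it.
; On Stage3_2 it shows the happy ending only if Countcat equals 3, otherwise the bad ending.
; A separate box plays a one-time meow.
; Tick destroys the cat when the game mode's CatNPC is false, with delayed widget removal, and Npcchatlog increments GI_stage chat counters per stage.
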(event OnComponentBeginOverlap(Capsule)
  (params (OverlappedComponent :type Primitive%20Component%20Object%20Reference) (OtherActor :type Actor%20Object%20Reference) (OtherComp :type Primitive%20Component%20Object%20Reference) (OtherBodyIndex :type Integer) (bFromSweep :type Boolean) (SweepResult :type Hit%20Result%20Structure%20%28by%20ref%29))
  (bind _asbp_super_side_scroller_main_character (Utilities|Casting|CastToBP_SuperSideScroller_MainCharacter OtherActor))
  (if (== (Variables|/Game/MainCharacter/Blueprints/BP_SuperSideScroller_MainCharacter.BP_SuperSideScroller_MainCharacter_C|GetmainCapsule _asbp_super_side_scroller_main_character) OtherComp)
    (if (Variables|Default|Getstage3)
      (if (== (Variables|/Game/MainCharacter/Blueprints/BP_SuperSideScroller_MainCharacter.BP_SuperSideScroller_MainCharacter_C|Getcountcat _asbp_super_side_scroller_main_character) 3)
        (bind _returnvalue (UserInterface|CreateWidget "/Game/NPC/WBP_happyendingDialogue.WBP_happyendingDialogue_C"))
        (UserInterface|Viewport|AddtoViewport _returnvalue 0)
        (else
          (bind _returnvalue_2 (UserInterface|CreateWidget "/Game/NPC/WBP_badendingDialogue.WBP_badendingDialogue_C"))
          (UserInterface|Viewport|AddtoViewport _returnvalue_2 0)))
      (else
        (bind _returnvalue_3 (UserInterface|CreateWidget "/Game/NPC/WBP_Dialogue1.WBP_Dialogue1_C"))
        (UserInterface|Viewport|AddtoViewport _returnvalue_3 0)))))

(event OnComponentBeginOverlap(Box)
  (params (OverlappedComponent :type Primitive%20Component%20Object%20Reference) (OtherActor :type Actor%20Object%20Reference) (OtherComp :type Primitive%20Component%20Object%20Reference) (OtherBodyIndex :type Integer) (bFromSweep :type Boolean) (SweepResult :type Hit%20Result%20Structure%20%28by%20ref%29))
  (if (== OtherActor (Game|Player|GetPlayerPawn 0))
    (Utilities|FlowControl|DoOnce false
      (:Completed
        (Audio|PlaySound2D "/Game/Sound/MeowSound.MeowSound" 1.0 1.0 0.0 0 0)))))

(event OnComponentEndOverlap(Box)
  (params (OverlappedComponent :type Primitive%20Component%20Object%20Reference) (OtherActor :type Actor%20Object%20Reference) (OtherComp :type Primitive%20Component%20Object%20Reference) (OtherBodyIndex :type Integer))
  (if (not (== OtherActor (Game|Player|GetPlayerPawn 0)))
    (Audio|Components|Audio|Stop (Variables|Default|GetAudio))))

(event EventBeginPlay
  (bind _returnvalue (Game|GetCurrentLevelName true))
  (Variables|Default|Setstage3 (Utilities|Enum|Equal(Enum) _returnvalue "Stage3_2")))

(event Collision|EventActorBeginOverlap
  (params (OtherActor :type Actor%20Object%20Reference)))

(event EventTick
  (params (DeltaSeconds :type Float%20%28single-precision%29))
  (bind _asboy_game_mode (Utilities|Casting|CastToBoyGameMode (Game|GetGameMode)))
  (if (not (Variables|/Game/MainCharacter/Blueprints/BoyGameMode.BoyGameMode_C|GetCatNPC _asboy_game_mode))
    (Actor|DestroyActor)
    (Utilities|FlowControl|Delay 2.0)
    (Widget|RemovefromParent (stale OnComponentBeginOverlap(Capsule) _returnvalue_3))
    (Widget|RemovefromParent (stale OnComponentBeginOverlap(Capsule) _returnvalue))
    (Widget|RemovefromParent (stale OnComponentBeginOverlap(Capsule) _returnvalue_2))))

(fn ConstructionScript)

(fn Npcchatlog
  (bind _asgi_stage (Utilities|Casting|CastToGI_stage (Game|GetGameInstance)))
  (Math|Integer|IncrementInt (Variables|/Game/MainCharacter/Blueprints/GI_stage.GI_stage_C|Getnpcchat _asgi_stage)
    (:%20%20
      (bind _returnvalue (Game|GetCurrentLevelName true))
      (if (Utilities|Enum|Equal(Enum) _returnvalue "Stage1_2")
        (bind _result (Math|Integer|IncrementInt (Variables|/Game/MainCharacter/Blueprints/GI_stage.GI_stage_C|Getnpcchat1 _asgi_stage))
          (:%20%20
            (Variables|/Game/MainCharacter/Blueprints/GI_stage.GI_stage_C|Setnpcchat1 _asgi_stage _result)))
        (elif (or (Utilities|Enum|Equal(Enum) _returnvalue "Stage2_2A") (Utilities|Enum|Equal(Enum) _returnvalue "Stage2_2B"))
          (Math|Integer|IncrementInt (Variables|/Game/MainCharacter/Blueprints/GI_stage.GI_stage_C|Getnpcchat2 _asgi_stage)
            (:%20%20
              _))
          (elif (Utilities|Enum|Equal(Enum) _returnvalue "Stage3_2")
            (Math|Integer|IncrementInt (Variables|/Game/MainCharacter/Blueprints/GI_stage.GI_stage_C|Getnpcchat3 _asgi_stage)
              (:%20%20
                _)))))
      (return))))