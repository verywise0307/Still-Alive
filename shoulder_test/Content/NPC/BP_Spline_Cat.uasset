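; BP_Spline_Cat is an NPC cat actor that moves its mesh along a spline at a set speed.
; Each Tick it advances a distance by SplineSpeed times delta time and samples the spline's local transform there to place CatMesh.
; Fixed offsets lower the mesh and correct its yaw, while its scale is preserved.
; When Loop is enabled, the distance resets to zero after passing the spline's end.
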(event EventTick
  (params (DeltaSeconds :type Float%20%28single-precision%29))
  (Variables|Default|SetDistance (+ (* DeltaSeconds (Variables|Default|GetSpline%20Speed)) (Variables|Default|GetDistance)))
  (Transformation|SetRelativeTransform (Variables|Default|GetCatMesh) (Math|Transform|MakeTransform (Math|Vector|MakeVector (.x (.location (Spline|GetTransformatDistanceAlongSpline (Variables|Default|GetSpline) (Variables|Default|GetDistance) "Local" false))) (.y (.location (Spline|GetTransformatDistanceAlongSpline (Variables|Default|GetSpline) (Variables|Default|GetDistance) "Local" false))) (+ (.z (.location (Spline|GetTransformatDistanceAlongSpline (Variables|Default|GetSpline) (Variables|Default|GetDistance) "Local" false))) -9e+01)) (Math|Rotator|MakeRotator (.roll (.rotation (Spline|GetTransformatDistanceAlongSpline (Variables|Default|GetSpline) (Variables|Default|GetDistance) "Local" false))) (.pitch (.rotation (Spline|GetTransformatDistanceAlongSpline (Variables|Default|GetSpline) (Variables|Default|GetDistance) "Local" false))) (+ (.yaw (.rotation (Spline|GetTransformatDistanceAlongSpline (Variables|Default|GetSpline) (Variables|Default|GetDistance) "Local" false))) -9e+01)) (Variables|/Script/Engine.SceneComponent|GetRelativeScale3D (Variables|Default|GetCatMesh))) false false)
  (if (Variables|Default|GetLoop)
    (if (> (Variables|Default|GetDistance) (Spline|GetSplineLength (Variables|Default|GetSpline)))
      (Variables|Default|SetDistance 0.0))))

(fn ConstructionScript)