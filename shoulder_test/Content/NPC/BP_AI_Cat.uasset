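; Cat NPC Blueprint that wanders on its own and chases the side-scroller's main character on sight.
; While no player is seen, Tick runs a randomly timed Delay, then moves the cat to a random reachable point nearby.
; PawnSensing sightings set a seen flag and start an AIMoveTo toward the player.
; A short retriggerable delay clears the flag once sightings stop, letting wandering resume.
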(event OnSeePawn(PawnSensing)
  (params (Pawn :type Pawn%20Object%20Reference))
  (bind _asbp_super_side_scroller_main_character (Utilities|Casting|CastToBP_SuperSideScroller_MainCharacter Pawn))
  (Utilities|FlowControl|Sequence
    (:then_0
      (Variables|Default|SetCanSeeEnenmy? true)
      (AI|AIMoveTo self "0, 0, 0" _asbp_super_side_scroller_main_character 5.0 false))
    (:then_1
      (Utilities|FlowControl|RetriggerableDelay 0.5)
      (Variables|Default|SetCanSeeEnenmy? false))))

(event EventTick
  (params (DeltaSeconds :type Float%20%28single-precision%29))
  (if (not (Variables|Default|GetCanSeeEnenmy?))
    (Utilities|FlowControl|Delay (Math|Random|RandomFloatinRange 2.0 6.0))
    (AI|AIMoveTo self (.RandomLocation (AI|Navigation|GetRandomReachablePointinRadius (Transformation|GetActorLocation) 2e+02 0 0)) 0 5.0 false)))

(fn ConstructionScript)